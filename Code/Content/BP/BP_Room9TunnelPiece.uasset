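; Tunnel segment for Room 9 that sits on a ring and carries a board, which can award a one-time bonus.
; SetPos places and rolls the piece by radius and twist angles, offsetting the board by its left/right ratios.
; SetThick scales it to the arc length and target cross-section.
; BeginPlay narrows DifficultyScene in Y by global difficulty, and a player hit on a bonus board calls the parent's ShowBonus.
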(event OnComponentHit(Board)
  (params (HitComponent :type Primitive%20Component%20Object%20Reference) (OtherActor :type Actor%20Object%20Reference) (OtherComp :type Primitive%20Component%20Object%20Reference) (NormalImpulse :type Vector :default "0, 0, 0") (Hit :type Hit%20Result%20Structure%20%28by%20ref%29))
  ;[1 1 1] Collection Check
  (if (== OtherActor (Game|GetPlayerCharacter 0))
    (if (Variables|Components|GetisBonus)
      (Default|ShowBonus (Variables|Components|GetParent))
      (Variables|Components|SetisBonus false))))

(event EventBeginPlay
  (bind _difficultyscene (Variables|Default|GetDifficultyScene))
  (bind _relativescale3d (Variables|/Script/Engine.SceneComponent|GetRelativeScale3D _difficultyscene))
  (bind (_x _y _z) (Math|Vector|BreakVector _relativescale3d))
  ;[1 1 1] Difficulty Setting
  (bind _asm_game_instance (Utilities|Casting|CastTomGameInstance (Game|GetGameInstance)))
  (Transformation|SetRelativeScale3D (Variables|Default|GetDifficultyScene) (Math|Vector|MakeVector _x (Utilities|Select :Index (Variables|/Game/UI/mGameInstance.mGameInstance_C|GetglobalDifficulty _asm_game_instance) :Option%200 1.0 :Option%201 0.6 :Option%202 0.25) _z)))

(fn ConstructionScript)

(fn SetPos
  (params (RadiusAngle :type Float%20%28single-precision%29) (SelfRotateAngle :type Float%20%28single-precision%29))
  (bind _returnvalue (* RadiusAngle -1.0))
  (bind _boardrightratio (Variables|Components|GetBoardRightRatio))
  (bind _boardleftratio (Variables|Components|GetBoardLeftRatio))
  (bind _returnvalue_2 (- _boardrightratio _boardleftratio))
  (Transformation|SetActorRelativeLocation (Math|Conversions|ToVector(Vector2D) (* (Math|Vector2D|MakeVector2D (Math|Trig|Cos(Degrees) _returnvalue) (Math|Trig|Sin(Degrees) _returnvalue)) (Variables|Components|GetRadius))))
  (Transformation|SetActorRelativeRotation (Math|Rotator|CombineRotators (Math|Vector|RotatorfromAxisandAngle "1.000000,0.000000,0.000000" (+ (* SelfRotateAngle -1.0) (Variables|Components|GetSelfRotateBaseAngle))) (Math|Vector|RotatorfromAxisandAngle "0,0.000000,1.000000" (+ _returnvalue 9e+01))))
  (Transformation|SetRelativeLocation (Variables|Default|GetBoard) (Math|Vector|MakeVector 0.0 (* (.Y (Math|Vector|BreakVector (Variables|/Script/Engine.SceneComponent|GetRelativeScale3D (Variables|Default|GetBoard)))) (.Y (Math|Vector|BreakVector (Variables|Components|GetTargetSize))) (- 0.5 (* _returnvalue_2 0.5)) (/ 1.0 _returnvalue_2)) 2.5e+02) false false))

(fn SetThick
  (params (Angle :type Float%20%28single-precision%29))
  (bind _meshsize (Variables|Components|GetMeshSize))
  (bind _targetsize (Variables|Components|GetTargetSize))
  (bind (_x _y _z) (Math|Vector|BreakVector _meshsize))
  (bind (_x_2 _y_2 _z_2) (Math|Vector|BreakVector _targetsize))
  (Transformation|SetRelativeScale3D (Variables|Default|GetDefaultSceneRoot) (Math|Vector|MakeVector (* (/ Angle 1.8e+02) (Math|Trig|GetPI) (Variables|Components|GetRadius) 1.0 (/ 1.0 _x)) (* (/ _y_2 _y) (- (Variables|Components|GetBoardRightRatio) (Variables|Components|GetBoardLeftRatio))) (/ _z_2 _z))))