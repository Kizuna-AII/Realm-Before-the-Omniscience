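; Outer ring piece of the Room 9 tunnel that calls PlayerRespawn on its Parent when hit.
; SetPos places it on a horizontal circle around Center, oriented along the tangent and rolled by a self-rotation angle.
; SetThick scales the cube so its length spans an arc angle at slightly padded radius, with width and height normalized from TargetSize by MeshSize.
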(event Collision|EventHit
  (params (MyComp :type Primitive%20Component%20Object%20Reference) (Other :type Actor%20Object%20Reference) (OtherComp :type Primitive%20Component%20Object%20Reference) (bSelfMoved :type Boolean) (HitLocation :type Vector :default "0, 0, 0") (HitNormal :type Vector :default "0, 0, 0") (NormalImpulse :type Vector :default "0, 0, 0") (Hit :type Hit%20Result%20Structure%20%28by%20ref%29))
  (Default|PlayerRespawn (Variables|Components|GetParent)))

(fn ConstructionScript)

(fn SetPos
  (params (RadiusAngle :type Float%20%28single-precision%29) (SelfRotateAngle :type Float%20%28single-precision%29))
  (Transformation|SetActorLocationAndRotation (+ (Math|Conversions|ToVector(Vector2D) (* (Math|Vector2D|MakeVector2D (Math|Trig|Cos(Degrees) RadiusAngle) (Math|Trig|Sin(Degrees) RadiusAngle)) (Variables|Components|GetRadius))) (Variables|Components|GetCenter)) (Math|Rotator|CombineRotators (Math|Vector|RotatorfromAxisandAngle "1.000000,0.000000,0.000000" SelfRotateAngle) (Math|Vector|RotatorfromAxisandAngle "0,0.000000,1.000000" (+ RadiusAngle 9e+01)))))

(fn SetThick
  (params (Angle :type Float%20%28single-precision%29))
  (bind _meshsize (Variables|Components|GetMeshSize))
  (bind _targetsize (Variables|Components|GetTargetSize))
  (bind (_x _y _z) (Math|Vector|BreakVector _meshsize))
  (bind (_x_2 _y_2 _z_2) (Math|Vector|BreakVector _targetsize))
  (Transformation|SetWorldScale3D (Variables|Default|GetCube) (Math|Vector|MakeVector (* (/ Angle 1.8e+02) (Math|Trig|GetPI) (+ (Variables|Components|GetRadius) (* _y_2 1.6125)) 1.0 (/ 1.0 _x)) (/ _y_2 _y) (/ _z_2 _z))))