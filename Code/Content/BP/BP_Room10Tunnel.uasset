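; Room 10 tunnel actor that spawns pieces along an arc around its root, twisted progressively over its length, with fairies at regular piece intervals in quarter-turn steps.
; UpdateView places every piece and fairy from radius angle and self-rotation, and sizes piece thickness to the arc.
; While the camera's angle falls within the arc, throttled Tick counter-rotates the whole twist so the piece at the camera has zero roll.
; Holding I manually advances the offset for testing.
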(event EventBeginPlay
  ;[1 1 1] Construction
  (for _index (range 0 (- (Variables|Components|GetTotalPieceNum) 1))
    (bind _returnvalue (Game|SpawnActorfromClass "/Game/BP/BP_Room10TunnelPiece.BP_Room10TunnelPiece_C" (Math|Transform|MakeTransform "0, 0, 0") "Undefined" 0 0))
    (Utilities|Array|Add (Variables|Components|GetPieces) _returnvalue)
    (if (== (Math|Integer|%(Integer) _index (Variables|Components|GetPiecesPerFairy)) 0)
      (bind _returnvalue_2 (Game|SpawnActorfromClass "/Game/BP/BP_Room10TunnelFairy.BP_Room10TunnelFairy_C" (Math|Transform|MakeTransform "0, 0, 0") "Undefined" 0 0))
      (Utilities|Array|Add (Variables|Components|GetFairyPieces) _returnvalue_2)))
  (CallFunction|UpdateView)
  (Utilities|FlowControl|Delay 0.5)
  (Variables|Components|SetSelfRotateOffsetAngle 0.0)
  (CallFunction|UpdateView))

(event EventTick
  (params (DeltaSeconds :type Float%20%28single-precision%29))
  (bind _returnvalue (Game|GetPlayerController 0))
  (bind _pieces (Variables|Components|GetPieces))
  (bind _output (Utilities|Array|Get(acopy) _pieces))
  (bind _playercameramanager (Variables|/Script/Engine.PlayerController|GetPlayerCameraManager _returnvalue))
  (bind _returnvalue_2 (Camera|GetCameraLocation _playercameramanager))
  (bind _center (Variables|/Game/BP/BP_Room10TunnelPiece.BP_Room10TunnelPiece_C|GetCenter _output))
  (bind _returnvalue_3 (- _returnvalue_2 _center))
  (bind (_x _y) (Math|Vector|BreakVector _returnvalue_3))
  (bind _returnvalue_4 (Class|KismetMathLibrary|DegAtan2 _y _x))
  ;[1 1 1] Test
  (if (Game|Player|IsInputKeyDown (Game|GetPlayerController 0) "I")
    (Variables|Components|SetSelfRotateOffsetAngle (+ (Variables|Components|GetSelfRotateOffsetAngle) 1.0))
    (CallFunction|UpdateView)
    (Development|PrintString (Utilities|String|ToString(Float) (Variables|Components|GetSelfRotateOffsetAngle))))
  (bind _output_get (Variables|Components|SetAccTime (+ DeltaSeconds (Variables|Components|GetAccTime))))
  (if (>= _output_get 0.01)
    (Variables|Components|SetAccTime 0.0)
    (if (not (== _output 0)) ; check whether empty
      (bind _isintunnel (CallFunction|CheckPlayerinTunnel _returnvalue_4))
      (if _isintunnel
        (Variables|Components|SetSelfRotateOffsetAngle (- 0.0 (Utilities|GetSelfRotateAngleWithoutOffset (Utilities|GetIndexfromRadiusAngle _returnvalue_4))))
        (CallFunction|UpdateView)))))

(fn ConstructionScript)

(fn UpdateView
  (for (_array_element _array_index) (Variables|Components|GetPieces)
    (Variables|/Game/BP/BP_Room10TunnelPiece.BP_Room10TunnelPiece_C|SetCenter _array_element (Transformation|GetWorldLocation (Variables|Default|GetDefaultSceneRoot)))
    (Default|SetPos _array_element (Utilities|GetRadiusAngle _array_index) (Utilities|GetSelfRotateAngle _array_index))
    (Default|SetThick _array_element (/ (Variables|Components|GetTotalRadiusAngle) (Math|Conversions|ToFloat(Integer) (Variables|Components|GetTotalPieceNum)))))
  (for (_array_element_2 _array_index_2) (Variables|Components|GetFairyPieces)
    (Variables|/Game/BP/BP_Room10TunnelFairy.BP_Room10TunnelFairy_C|SetCenter _array_element_2 (Transformation|GetWorldLocation (Variables|Default|GetDefaultSceneRoot)))
    (Default|SetPos _array_element_2 (Utilities|GetRadiusAngle (* _array_index_2 (Variables|Components|GetPiecesPerFairy))) (+ (Utilities|GetSelfRotateAngle (* _array_index_2 (Variables|Components|GetPiecesPerFairy))) (* _array_index_2 9e+01)))))

(fn CheckPlayerinTunnel
  (params (RelativeAngle :type Float%20%28single-precision%29))
  (bind _startangle (Variables|Components|GetStartAngle))
  (bind _totalradiusangle (Variables|Components|GetTotalRadiusAngle))
  (bind _returnvalue (+ _startangle _totalradiusangle))
  (return (or (and (>= RelativeAngle _startangle) (<= RelativeAngle _returnvalue)) (<= RelativeAngle (- _returnvalue 3.6e+02)))))