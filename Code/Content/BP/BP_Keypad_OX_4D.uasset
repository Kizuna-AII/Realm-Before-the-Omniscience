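; A four-digit O/X keypad lock that opens its bound Door when the button pattern matches Password.
; On BeginPlay it spawns a centered row of BP_KeypadButton_OX actors set to O, each storing the keypad and its index.
; While locked, ChangeNumber toggles a button between O and X, then compares the concatenated button states to Password.
; E and F are test keys that force the door open/unlocked or closed/locked.
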(event EventBeginPlay
  (CallFunction|AddButton 4))

(event Input|KeyboardEvents|E
  (params (Key :type Key%20Structure :default "None"))
  ;[1 1 1] Test
  (:Pressed
    (Development|PrintString "Press E")
    (Default|OpenDoor (Variables|Components|GetDoor))
    (Variables|Components|SetisLocked false)))

(event Input|KeyboardEvents|F
  (params (Key :type Key%20Structure :default "None"))
  ;[1 1 1] Test
  (:Pressed
    (Development|PrintString "Press F")
    (Default|CloseDoor (Variables|Components|GetDoor))
    (Variables|Components|SetisLocked true)))

(fn ConstructionScript)

(fn ChangeNumber
  (params (Index :type Integer))
  (bind _door (Variables|Components|GetDoor))
  (bind _buttons (Variables|Components|GetButtons))
  (bind _output (Utilities|Array|Get(acopy) _buttons Index))
  (if (Variables|Components|GetisLocked)
    (switch string (Variables|/Game/BP/BP_KeypadButton_OX.BP_KeypadButton_OX_C|GetNumber _output)
      (:O
        (Default|SetNumber _output "X" false))
      (:X
        (Default|SetNumber _output "O" false)))
    (bind _password (CallFunction|GetInputPassword))
    (if (Utilities|Enum|Equal(Enum) _password (Variables|Components|GetPassword))
      (Variables|Components|SetisLocked false)
      (if (== _door 0)
        (Development|PrintString "Lock is unlocked, but no binding door")
        (else
          (Default|OpenDoor _door)
          (Development|PrintString "Password Correct."))))))

(fn GetInputPassword
  (for _array_element (Variables|Components|GetButtons)
    (LocalVariables|SetRes (Utilities|String|Append (LocalVariables|GetRes) (Variables|/Game/BP/BP_KeypadButton_OX.BP_KeypadButton_OX_C|GetNumber _array_element))))
  (return (LocalVariables|GetRes)))

(fn AddButton
  (params (NumOfDigits :type Integer))
  (bind _returnvalue (- NumOfDigits 1))
  (bind _buttons (Variables|Components|GetButtons))
  ;[1 1 1] Construct Buttons
  (for _index (range 0 _returnvalue)
    (bind _returnvalue_2 (Game|SpawnActorfromClass "/Game/BP/BP_KeypadButton_OX.BP_KeypadButton_OX_C" (Math|Transform|MakeTransform "0, 0, 0") "Undefined" 0 0))
    (bind _returnvalue_3 (Utilities|Array|Add _buttons _returnvalue_2))
    (Variables|/Game/BP/BP_KeypadButton_OX.BP_KeypadButton_OX_C|SetOldParent (Utilities|Array|Get(acopy) _buttons _returnvalue_3) self)
    (Variables|/Game/BP/BP_KeypadButton_OX.BP_KeypadButton_OX_C|SetIndexInParent (Utilities|Array|Get(acopy) _buttons _returnvalue_3) _returnvalue_3)
    (Default|SetNumber (Utilities|Array|Get(acopy) _buttons _returnvalue_3) "O" false)
    (Default|SetCoord (Utilities|Array|Get(acopy) _buttons _returnvalue_3) (Math|Vector2D|MakeVector2D (- (Math|Conversions|ToFloat(Integer) _returnvalue_3) (/ (Math|Conversions|ToFloat(Integer) _returnvalue) 2.0)) 0.0))))