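; Flashlight board actor that lets the player move a child flashlight across it with the keyboard while the board is selected.
; On BeginPlay it links its child button back to itself, caches the flashlight and fires an initial move update to the flashlight's current position.
; I, L, K and J pass four direction indices to the flashlight's TryToMove, gated by a flag that Select and Unselect set.
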(event EventBeginPlay
  (bind _asbp_flashlight_button (Utilities|Casting|CastToBP_Flashlight_Button (Variables|/Script/Engine.ChildActorComponent|GetChildActor (Variables|Default|GetButton))))
  (Variables|/Game/BP/BP_Flashlight_Button.BP_Flashlight_Button_C|SetParent _asbp_flashlight_button self)
  (bind _asbp_flashlight (Utilities|Casting|CastToBP_flashlight (Variables|/Script/Engine.ChildActorComponent|GetChildActor (Variables|Default|GetFlashlight))))
  (bind _output_get (Variables|Components|SetFlashLightActor _asbp_flashlight))
  (Default|CallOnMove :self _output_get :NewPos (Variables|/Game/BP/BP_flashlight.BP_flashlight_C|GetPos _output_get)))

(event Input|KeyboardEvents|J
  (params (Key :type Key%20Structure :default "None"))
  (:Pressed
    (if (Variables|Components|GetSelected)
      (Default|TrytoMove (Variables|Components|GetFlashLightActor) 3))))

(event Input|KeyboardEvents|K
  (params (Key :type Key%20Structure :default "None"))
  (:Pressed
    (if (Variables|Components|GetSelected)
      (Default|TrytoMove (Variables|Components|GetFlashLightActor) 2))))

(event Input|KeyboardEvents|L
  (params (Key :type Key%20Structure :default "None"))
  (:Pressed
    (if (Variables|Components|GetSelected)
      (Default|TrytoMove (Variables|Components|GetFlashLightActor) 1))))

(event Input|KeyboardEvents|I
  (params (Key :type Key%20Structure :default "None"))
  (:Pressed
    (if (Variables|Components|GetSelected)
      (Default|TrytoMove (Variables|Components|GetFlashLightActor)))))

(fn ConstructionScript
  (|CallParentFunction))

(fn Unselect
  (Variables|Components|SetSelected false))

(fn Select
  (Variables|Components|SetSelected true))