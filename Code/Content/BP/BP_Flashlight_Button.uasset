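; Flashlight button Blueprint that responds to being hovered and exposes its name.
; Mouse-over and mouse-out events toggle custom depth rendering on its Cube and call Select or Unselect on its Parent reference.
; GetName returns the stored Name, and the construction script only runs the inherited one.
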(event EventOnMouseUnfover
  (Rendering|SetRenderCustomDepth (Variables|Default|GetCube) false)
  (Default|Unselect (Variables|Components|GetParent)))

(event EventOnMouseFover
  (Rendering|SetRenderCustomDepth (Variables|Default|GetCube) true)
  (Default|Select (Variables|Components|GetParent)))

(fn ConstructionScript
  (|CallParentFunction))

(fn GetName
  (return (Variables|Default|GetName)))