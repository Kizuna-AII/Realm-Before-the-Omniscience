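; BP_SoundManager is a sound manager that plays 2D sounds under shared global volume and pitch settings.
; Named sounds are stored in a name-to-component map, so a name still playing is not started again and can be killed by name.
; Unnamed sounds are spawned without tracking.
; Volume and pitch changes update the globals and all valid tracked sounds, leaving untracked ones already playing unchanged.
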(fn ConstructionScript)

(fn PlaySoundwithName
  (params (sound :type Sound%20Base%20Object%20Reference) (name :type String))
  (bind _soundmap (Variables|Components|GetSoundMap))
  (bind (_value _returnvalue) (Utilities|Map|Find _soundmap name))
  (if _returnvalue ; check whether name existance
    (if (Utilities|IsValid _value) ; check whether destroyed
      (if (Audio|Components|Audio|IsPlaying _value) ; check whether playing
        (return false)
        (else
          _))))
  (bind _returnvalue_2 (Audio|SpawnSound2D sound (Variables|Default|GetGlobalVolume) (Variables|Default|GetGlobalPitch) 0.0 0))
  (Utilities|Map|Add (Variables|Components|GetSoundMap) name _returnvalue_2)
  (return true))

(fn KillSoundfromName
  (params (Name :type String))
  (bind _soundmap (Variables|Components|GetSoundMap))
  (bind (_value _returnvalue) (Utilities|Map|Find _soundmap Name))
  (if _returnvalue ; check whether name existance
    (if (Utilities|IsValid _value) ; check whether destroyed
      (Components|DestroyComponent _value)
      (Utilities|Map|Remove (Variables|Components|GetSoundMap) Name)
      (Development|PrintString "Remove Success"))))

(fn PlaySoundWithoutName
  (params (sound :type Sound%20Base%20Object%20Reference) (name :type String))
  (Audio|SpawnSound2D sound (Variables|Default|GetGlobalVolume) (Variables|Default|GetGlobalPitch) 0.0 0))

(fn AdjustVolume
  (params (Volume :type Float%20%28single-precision%29))
  (Variables|Default|SetGlobalVolume Volume)
  (bind _values (Utilities|Map|Values (Variables|Components|GetSoundMap)))
  (for _array_element _values
    (if (Utilities|IsValid _array_element)
      (Audio|Components|Audio|SetVolumeMultiplier _array_element (Variables|Default|GetGlobalVolume) :!class /Script/Engine.AudioComponent))))

(fn AdjustPitch
  (params (Pitch :type Float%20%28single-precision%29))
  (Variables|Default|SetGlobalPitch Pitch)
  (bind _values (Utilities|Map|Values (Variables|Components|GetSoundMap)))
  (for _array_element _values
    (if (Utilities|IsValid _array_element)
      (Audio|Components|Audio|SetPitchMultiplier _array_element (Variables|Default|GetGlobalPitch)))))

(fn GetVolume
  (return (Variables|Default|GetGlobalVolume)))

(fn GetPitch
  (return (Variables|Default|GetGlobalPitch)))