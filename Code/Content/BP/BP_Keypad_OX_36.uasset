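; BP_Keypad_OX_36 is a keypad variant that builds 36 O/X buttons in centred rows of 16, 4 and 16.
; AddButtonWithY spawns each BP_KeypadButton_OX, stores it in Buttons, and sets its parent, index and grid coordinate.
; The Changeable array decides whether a button starts as an editable "O" or shows its fixed character from the Password string.
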(event EventBeginPlay)

(event Collision|EventActorBeginOverlap
  (params (OtherActor :type Actor%20Object%20Reference)))

(event EventTick
  (params (DeltaSeconds :type Float%20%28single-precision%29)))

(fn ConstructionScript
  (|CallParentFunction))

(fn AddButton36
  ;[1 1 1] Construct Buttons
  (CallFunction|AddButtonwithY 16 2.0)
  (CallFunction|AddButtonwithY 4 1.0)
  (CallFunction|AddButtonwithY 16 0.0))

(fn AddButtonwithY
  (params (NumberOfButton :type Integer) (Y :type Float%20%28single-precision%29))
  (bind _returnvalue (- NumberOfButton 1))
  (bind _buttons (Variables|Default|GetButtons))
  ;[1 1 1] Construct Buttons
  (for _index (range 0 _returnvalue)
    (bind _returnvalue_2 (Game|SpawnActorfromClass "/Game/BP/BP_KeypadButton_OX.BP_KeypadButton_OX_C" (Math|Transform|MakeTransform "0, 0, 0") "Undefined" 0 0))
    (bind _returnvalue_3 (Utilities|Array|Add _buttons _returnvalue_2))
    (Variables|/Game/BP/BP_KeypadButton_OX.BP_KeypadButton_OX_C|SetParent (Utilities|Array|Get(acopy) _buttons _returnvalue_3) self)
    (Variables|/Game/BP/BP_KeypadButton_OX.BP_KeypadButton_OX_C|SetIndexInParent (Utilities|Array|Get(acopy) _buttons _returnvalue_3) _returnvalue_3)
    (Default|SetChangeable (Utilities|Array|Get(acopy) _buttons _returnvalue_3) (Utilities|Array|Get(acopy) (Variables|Default|GetChangeable) _returnvalue_3))
    (if (Utilities|Array|Get(acopy) (Variables|Default|GetChangeable) _returnvalue_3)
      (Default|SetNumber (Utilities|Array|Get(acopy) _buttons _returnvalue_3) "O" (Utilities|Array|Get(acopy) (Variables|Default|GetChangeable) _returnvalue_3))
      (else
        (Default|SetNumber (Utilities|Array|Get(acopy) _buttons _returnvalue_3) (Utilities|String|GetSubstring (Variables|Default|GetPassword) _returnvalue_3) (Utilities|Array|Get(acopy) (Variables|Default|GetChangeable) _returnvalue_3))))
    (Default|SetCoord (Utilities|Array|Get(acopy) _buttons _returnvalue_3) (Math|Vector2D|MakeVector2D (- (Math|Conversions|ToFloat(Integer) _index) (/ (Math|Conversions|ToFloat(Integer) _returnvalue) 2.0)) Y))))