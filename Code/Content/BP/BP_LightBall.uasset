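; BP_LightBall is a clickable ball actor that cycles its sphere through a list of materials.
; The construction script applies the first material, and ChangeColor advances a wrapping index to set the next one.
; Hovering toggles custom depth on the sphere, likely for a highlight, and a click calls ChangeColor only when MouseToChange is enabled.
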(event EventOnMouseUnfover
  (Rendering|SetRenderCustomDepth (Variables|Default|GetSphere) false))

(event EventOnMouseFover
  (Rendering|SetRenderCustomDepth (Variables|Default|GetSphere) true))

(event EventOnMouseClicked
  (if (Variables|组件|GetMouseToChange)
    (CallFunction|ChangeColor)))

(fn ConstructionScript
  (Rendering|Material|SetMaterial (Variables|Default|GetSphere) 0 (Utilities|Array|Get(acopy) (Variables|组件|GetMaterials))))

(fn ChangeColor
  (bind _materials (Variables|组件|GetMaterials))
  (bind _output_get (Variables|Components|SetColorNow (Math|Integer|%(Integer) (+ (Variables|Components|GetColorNow) 1) (Utilities|Array|Length _materials))))
  (Rendering|Material|SetMaterial (Variables|Default|GetSphere) 0 (Utilities|Array|Get(acopy) _materials _output_get)))