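; Test actor whose Cube component moves under a simulated gravity that can be flipped.
; Every Tick adds GravityScale, negated while IsReverse is set, to the Cube's physics linear velocity without delta-time scaling, so the acceleration depends on frame rate.
; The G key is a test binding that calls Reverse, which toggles IsReverse and prints a message.
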(event EventBeginPlay)

(event EventTick
  (params (DeltaSeconds :type Float%20%28single-precision%29))
  ;[1 1 1] Simulate Gravity
  (bind _gravity (CallFunction|GetGravity))
  (Physics|SetPhysicsLinearVelocity (Variables|Default|GetCube) _gravity true "None"))

(event Input|KeyboardEvents|G
  (params (Key :type Key%20Structure :default "None"))
  ;[1 1 1] Test
  (:Pressed
    (CallFunction|Reverse)))

(fn ConstructionScript)

(fn GetGravity
  (bind _gravityscale (Variables|Components|GetGravityScale))
  (if (Variables|Components|GetisReverse)
    (return (* _gravityscale -1.0))
    (else
      (return _gravityscale))))

(fn Reverse
  (Variables|Components|SetisReverse (not (Variables|Components|GetisReverse)))
  (Development|PrintString "Reversed"))