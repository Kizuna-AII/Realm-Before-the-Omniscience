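; BP_MyPostEffect toggles the scene between color and gray and also handles camera-aimed interaction with pickupable actors.
; A timeline played or reversed drives PostProcess saturation, triggered by an event or the O key when control is enabled, with dispatchers announcing each change.
; Visibility line traces from the camera send click messages and, while P-toggled highlighting is on, hover/unhover calls, tracking the last hovered actor.
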(event Custom|ChangeColorState_Event
  ;[1 1 1] Gray Effect
  (bind _output_get (Variables|组件|SetColorState (not (Variables|组件|GetColorState))))
  (if _output_get
    (Default|CallChangetoColor)
    (bind _newtrack_0 (Timeline|Timeline_Gray Play)
      (:Update
        (Utilities|Struct|SetmembersinPostProcessSettings (Variables|/Script/Engine.PostProcessComponent|GetSettings (Variables|Default|GetPostProcess)) (Math|Vector4|MakeVector4 _newtrack_0 _newtrack_0 _newtrack_0 1.0))))
    (else
      (Default|CallChangetoGray)
      (Timeline|Timeline_Gray Reverse))))

(event EventBeginPlay
  (Utilities|FlowControl|Sequence
    (:then_0
      (Utilities|Struct|SetmembersinPostProcessSettings (Variables|/Script/Engine.PostProcessComponent|GetSettings (Variables|Default|GetPostProcess)) (select (Variables|组件|GetColorState) (Math|Vector4|MakeVector4 1.0 1.0 1.0 1.0) (Math|Vector4|MakeVector4 0.0 0.0 0.0 1.0))))
    (:then_1
      ;[1 1 1] Gray Effect
      (bind _newtrack_0 (Timeline|Timeline_Gray SetNewTime)
        (:Update
          (Utilities|Struct|SetmembersinPostProcessSettings (Variables|/Script/Engine.PostProcessComponent|GetSettings (Variables|Default|GetPostProcess)) (Math|Vector4|MakeVector4 _newtrack_0 _newtrack_0 _newtrack_0 1.0)))))))

(event EventTick
  (params (DeltaSeconds :type Float%20%28single-precision%29))
  (bind _returnvalue (Game|GetPlayerController 0))
  (bind _playercameramanager (Variables|/Script/Engine.PlayerController|GetPlayerCameraManager _returnvalue))
  (bind _returnvalue_2 (Camera|GetCameraLocation _playercameramanager))
  ;[1 1 1] Mouse Fover
  (if (Variables|Components|GetisHighlight)
    (bind (_outhit _returnvalue_3) (Collision|LineTraceByChannel _returnvalue_2 (+ _returnvalue_2 (* (Math|Rotator|GetRotationXVector (Camera|GetCameraRotation _playercameramanager)) 2e+04)) "TraceTypeQuery1" false 0 "None"))
    (if _returnvalue_3
      (bind _asbp_actor_pickupable (Utilities|Casting|CastToBP_Actor_Pickupable (.HitActor (Collision|BreakHitResult _outhit)))
        (:then
          (if (not (== (Variables|Components|GetLastPickupActor) _asbp_actor_pickupable)) ; new pickupable and different from formal one
            (Default|OnMouseFover _asbp_actor_pickupable)
            (if (== (Variables|Components|GetLastPickupActor) 0) :!label _label
              _
              (else
                (Default|OnMouseUnfover (Variables|Components|GetLastPickupActor)) ; cancel formal one
              ))
            (Variables|Components|SetLastPickupActor _asbp_actor_pickupable) ; save formal one
          ))
        (:CastFailed
          (goto _label))))))

(event Input|KeyboardEvents|O
  (params (Key :type Key%20Structure :default "None"))
  ;[1 1 1] Gray Effect
  (:Pressed
    (if (Variables|组件|GetEnableControl)
      (bind _output_get (Variables|组件|SetColorState (not (Variables|组件|GetColorState))))
      (if _output_get
        (Default|CallChangetoColor)
        (bind _newtrack_0 (Timeline|Timeline_Gray Play)
          (:Update
            (Utilities|Struct|SetmembersinPostProcessSettings (Variables|/Script/Engine.PostProcessComponent|GetSettings (Variables|Default|GetPostProcess)) (Math|Vector4|MakeVector4 _newtrack_0 _newtrack_0 _newtrack_0 1.0))))
        (else
          (Default|CallChangetoGray)
          (Timeline|Timeline_Gray Reverse))))))

(event Input|KeyboardEvents|P
  (params (Key :type Key%20Structure :default "None"))
  ;[1 1 1] Mouse Fover
  (:Pressed
    (Variables|Components|SetisHighlight (not (Variables|Components|GetisHighlight)))))

(event Input|MouseEvents|LeftMouseButton
  (params (Key :type Key%20Structure :default "None"))
  (bind _returnvalue (Game|GetPlayerController 0))
  (bind _playercameramanager (Variables|/Script/Engine.PlayerController|GetPlayerCameraManager _returnvalue))
  (bind _returnvalue_2 (Camera|GetCameraLocation _playercameramanager))
  ;[1 1 1] mouse click
  (:Pressed
    (bind (_outhit _returnvalue_3) (Collision|LineTraceByChannel _returnvalue_2 (+ _returnvalue_2 (* (Math|Rotator|GetRotationXVector (Camera|GetCameraRotation _playercameramanager)) 2e+04)) "TraceTypeQuery1" false 0 "None"))
    (if _returnvalue_3
      (bind _asbp_actor_pickupable (Utilities|Casting|CastToBP_Actor_Pickupable (.HitActor (Collision|BreakHitResult _outhit)))
        (:then
          (Class|BPIClickable|OnMouseClicked(Message) _asbp_actor_pickupable))
        (:CastFailed
          (Development|PrintString (Utilities|String|Append "name:" (Utilities|GetObjectName (.HitActor (Collision|BreakHitResult _outhit))) "Nonclickable")))))))

(fn ConstructionScript)