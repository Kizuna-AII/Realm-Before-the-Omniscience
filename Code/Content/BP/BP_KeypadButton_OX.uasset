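; BP_KeypadButton_OX is a clickable O/X button in a parent keypad that asks the parent to change its number when changeable.
; SetNumber picks the cube material from the O or X value and whether it is changeable.
; SetCoord fires a dispatcher whose timeline lerps between old and new coords, transforming them by the parent's matrix so the button follows its position, rotation and scale.
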(event Custom|OnSetCoord_Event
  (params (TargetCoord :type Vector) (OldCoord :type Vector))
  (bind _parent (Variables|Components|GetParent))
  ;[1 1 1] Process SetCoord Timeline Effect
  (bind _newtrack_0 (Timeline|Timeline_0 PlayFromStart)
    (:Update
      (Transformation|SetActorLocationAndRotation (Math|Conversions|ToVector(Vector4) (Class|KismetMathLibrary|TransformVector4 (Math|Transform|ToMatrix(Transform) (Transformation|GetActorTransform _parent)) (Math|Vector4|MakeVector4 (.X (Math|Vector|BreakVector (Math|Vector|Lerp(Vector) OldCoord TargetCoord _newtrack_0))) (.Y (Math|Vector|BreakVector (Math|Vector|Lerp(Vector) OldCoord TargetCoord _newtrack_0))) (.Z (Math|Vector|BreakVector (Math|Vector|Lerp(Vector) OldCoord TargetCoord _newtrack_0))) 1.0))) (Transformation|GetActorRotation _parent))
      (Transformation|SetActorScale3D (Transformation|GetActorScale3D _parent)))))

(event EventBeginPlay
  ;[1 1 1] Process SetCoord Timeline Effect
  (EventDispatchers|BindEventtoOnSetCoord (delegate Custom|OnSetCoord_Event)))

(event EventOnMouseClicked
  ;[1 1 1] click event
  (Development|PrintString "Clicked")
  (if (Variables|Default|GetChangeable)
    (Default|ChangeNumber (Variables|Components|GetParent) (Variables|Components|GetIndexInParent))
    (else
      (Development|PrintString "Unchangeable"))))

(fn ConstructionScript)

(fn SetNumber
  (params (Number :type String) (Changeable :type Boolean))
  (bind _cube (Variables|Default|GetCube))
  (bind _output_get (Variables|Components|SetNumber Number))
  (switch string _output_get
    (:O
      (if Changeable
        (Rendering|Material|SetMaterial _cube 0 "/Game/Material/Number/O_Mat_nT.O_Mat_NT")
        (else
          (Rendering|Material|SetMaterial _cube 0 "/Game/Material/Number/O_Mat.O_Mat"))))
    (:X
      (if Changeable
        (Rendering|Material|SetMaterial _cube 0 "/Game/Material/Number/X_Mat_NT.X_Mat_NT")
        (else
          (Rendering|Material|SetMaterial _cube 0 "/Game/Material/Number/X_Mat.X_Mat"))))))

(fn SetCoord
  (params (Coord :type Vector%202D%20Structure))
  (bind _output_get (LocalVariables|SetOldCoord (Variables|Components|GetCoord)))
  (bind _output_get_2 (Variables|Components|SetCoord Coord))
  (Default|CallOnSetCoord (Utilities|ConvertRealCoord _output_get_2) (Utilities|ConvertRealCoord _output_get)))

(fn SetChangeable
  (params (Changeable :type Boolean))
  (Variables|Default|SetChangeable Changeable))