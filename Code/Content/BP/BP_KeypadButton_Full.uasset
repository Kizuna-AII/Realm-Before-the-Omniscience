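; Keypad button actor that shows a digit or letter A–H, reports clicks to its parent keypad and toggles custom depth on hover.
; SetNumber swaps the cube's material to match the character.
; SetCoord fires a dispatcher with old and target coordinates passed through ConvertRealCoord, driving a timeline that slides the button between them in the parent's space, matching its rotation and scale.
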(event Custom|OnSetCoord_Event
  (params (TargetCoord :type Vector) (OldCoord :type Vector))
  (bind _parent (Variables|Components|GetParent))
  ;[1 1 1] Process SetCoord Timeline Effect
  (bind _newtrack_0 (Timeline|Timeline_0 PlayFromStart)
    (:Update
      (Transformation|SetActorLocationAndRotation (Math|Conversions|ToVector(Vector4) (Class|KismetMathLibrary|TransformVector4 (Math|Transform|ToMatrix(Transform) (Transformation|GetActorTransform _parent)) (Math|Vector4|MakeVector4 (.X (Math|Vector|BreakVector (Math|Vector|Lerp(Vector) OldCoord TargetCoord _newtrack_0))) (.Y (Math|Vector|BreakVector (Math|Vector|Lerp(Vector) OldCoord TargetCoord _newtrack_0))) (.Z (Math|Vector|BreakVector (Math|Vector|Lerp(Vector) OldCoord TargetCoord _newtrack_0))) 1.0))) (Transformation|GetActorRotation _parent))
      (Transformation|SetActorScale3D (Transformation|GetActorScale3D _parent)))))

(event EventOnMouseUnfover
  ;[1 1 1] click event
  (Rendering|SetRenderCustomDepth (Variables|Default|GetCube) false))

(event EventOnMouseClicked
  ;[1 1 1] click event
  (Development|PrintString "Clicked")
  (Default|ChangeNumber (Variables|Components|GetParent) (Variables|Components|GetIndexInParent)))

(event EventBeginPlay
  ;[1 1 1] Process SetCoord Timeline Effect
  (EventDispatchers|BindEventtoOnSetCoord (delegate Custom|OnSetCoord_Event)))

(event EventOnMouseFover
  ;[1 1 1] click event
  (Rendering|SetRenderCustomDepth (Variables|Default|GetCube) true))

(fn ConstructionScript)

(fn SetNumber
  (params (Number :type String))
  (bind _cube (Variables|Default|GetCube))
  (bind _cube_2 (Variables|Default|GetCube))
  (bind _output_get (Variables|Components|SetNumber Number))
  (switch string _output_get
    (:0
      ;[1 1 1] Number
      (Rendering|Material|SetMaterial _cube_2 0 "/Game/Material/Number/0_Mat_NT.0_Mat_NT"))
    (:1
      (Rendering|Material|SetMaterial _cube_2 0 "/Game/Material/Number/1_Mat_NT.1_Mat_NT"))
    (:2
      (Rendering|Material|SetMaterial _cube_2 0 "/Game/Material/Number/2_Mat_NT.2_Mat_NT"))
    (:3
      (Rendering|Material|SetMaterial _cube_2 0 "/Game/Material/Number/3_Mat_NT.3_Mat_NT"))
    (:4
      (Rendering|Material|SetMaterial _cube_2 0 "/Game/Material/Number/4_Mat_NT.4_Mat_NT"))
    (:5
      (Rendering|Material|SetMaterial _cube_2 0 "/Game/Material/Number/5_Mat_NT.5_Mat_NT"))
    (:6
      (Rendering|Material|SetMaterial _cube_2 0 "/Game/Material/Number/6_Mat_NT.6_Mat_NT"))
    (:7
      (Rendering|Material|SetMaterial _cube_2 0 "/Game/Material/Number/7_Mat_NT.7_Mat_NT"))
    (:8
      (Rendering|Material|SetMaterial _cube_2 0 "/Game/Material/Number/8_Mat_NT.8_Mat_NT"))
    (:9
      (Rendering|Material|SetMaterial _cube_2 0 "/Game/Material/Number/9_Mat_NT.9_Mat_NT"))
    (:A
      ;[1 1 1] Char
      (Rendering|Material|SetMaterial _cube 0 "/Game/Material/Number/A_Mat_NT.A_Mat_NT"))
    (:B
      (Rendering|Material|SetMaterial _cube 0 "/Game/Material/Number/B_Mat_NT.B_Mat_NT"))
    (:C
      (Rendering|Material|SetMaterial _cube 0 "/Game/Material/Number/C_Mat_NT.C_Mat_NT"))
    (:D
      (Rendering|Material|SetMaterial _cube 0 "/Game/Material/Number/D_Mat_NT.D_Mat_NT"))
    (:E
      (Rendering|Material|SetMaterial _cube 0 "/Game/Material/Number/E_Mat_NT.E_Mat_NT"))
    (:F
      (Rendering|Material|SetMaterial _cube 0 "/Game/Material/Number/F_Mat_NT.F_Mat_NT"))
    (:G
      (Rendering|Material|SetMaterial _cube 0 "/Game/Material/Number/G_Mat_NT.G_Mat_NT"))
    (:H
      (Rendering|Material|SetMaterial _cube 0 "/Game/Material/Number/H_Mat_NT.H_Mat_NT"))))

(fn SetCoord
  (params (Coord :type Vector%202D%20Structure))
  (bind _output_get (LocalVariables|SetOldCoord (Variables|Components|GetCoord)))
  (bind _output_get_2 (Variables|Components|SetCoord Coord))
  (Default|CallOnSetCoord (Utilities|ConvertRealCoord _output_get_2) (Utilities|ConvertRealCoord _output_get)))