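; Double-button piece for the Room 6 puzzle, placed and oriented relative to a parent actor.
; SetCoord fires a dispatcher whose timeline lerps the piece between old and new coordinates in the parent's space, applying ExpandDir yaw and parent-relative scale.
; When selectable, clicks request valid directions from the parent, while hover toggles parent selection and custom-depth highlighting.
; ChangeMesh swaps the cylinder's mesh and material.
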(event Custom|OnSetCoord_Event
  (params (TargetCoord :type Vector) (OldCoord :type Vector))
  (bind _parent (Variables|Components|GetParent))
  (bind _output (Utilities|ResolveSoftReference _parent))
  ;[1 1 1] Process SetCoord Timeline Effect
  (bind _newtrack_0 (Timeline|Timeline_0 PlayFromStart)
    (:Update
      (Transformation|SetActorLocationAndRotation (Math|Conversions|ToVector(Vector4) (Class|KismetMathLibrary|TransformVector4 (Math|Transform|ToMatrix(Transform) (Transformation|GetActorTransform _output)) (Math|Vector4|MakeVector4 (.X (Math|Vector|BreakVector (Math|Vector|Lerp(Vector) OldCoord TargetCoord _newtrack_0))) (.Y (Math|Vector|BreakVector (Math|Vector|Lerp(Vector) OldCoord TargetCoord _newtrack_0))) (.Z (Math|Vector|BreakVector (Math|Vector|Lerp(Vector) OldCoord TargetCoord _newtrack_0))) 1.0))) (Math|Rotator|CombineRotators (Math|Vector|RotatorfromAxisandAngle "0,0.000000,1.000000" (+ (* (Variables|Components|GetExpandDir) 9e+01) 2.7e+02)) (Transformation|GetActorRotation _output)))
      (Transformation|SetActorScale3D (* (* (Transformation|GetActorScale3D _output) "1.000000,1.000000,1.000000") (Variables|组件|GetScale))))))

(event EventBeginPlay
  ;[1 1 1] Process SetCoord Timeline Effect
  (EventDispatchers|BindEventtoOnSetCoord (delegate Custom|OnSetCoord_Event)))

(event EventOnMouseClicked
  ;[1 1 1] Process Mouse Event
  (if (Variables|Components|GetSelectable)
    (Default|GetDoubleButtonValidDirection (Utilities|ResolveSoftReference (Variables|Components|GetParent)) (Variables|Components|GetIndexInParent))))

(event EventOnMouseFover
  ;[1 1 1] Process Mouse Event
  (if (Variables|Components|GetSelectable)
    (Default|SelectDoubleButton (Utilities|ResolveSoftReference (Variables|Components|GetParent)) (Variables|Components|GetIndexInParent))
    (Rendering|SetRenderCustomDepth (Variables|Default|GetCylinder) true)))

(event EventOnMouseUnfover
  ;[1 1 1] Process Mouse Event
  (if (Variables|Components|GetSelectable)
    (Default|UnselectDoubleButton (Utilities|ResolveSoftReference (Variables|Components|GetParent)) (Variables|Components|GetIndexInParent))
    (Rendering|SetRenderCustomDepth (Variables|Default|GetCylinder) false)))

(fn ConstructionScript)

(fn SetCoord
  (params (Coord :type Vector%202D%20Structure))
  (bind _output_get (LocalVariables|SetOldCoord (Variables|Components|GetCoord)))
  (bind _output_get_2 (Variables|Components|SetCoord Coord))
  (Default|CallOnSetCoord (Utilities|ConvertRealCoord _output_get_2) (Utilities|ConvertRealCoord _output_get)))

(fn ChangeMesh
  (params (DButtonMesh :type Static%20Mesh%20Object%20Reference) (DButtonMat :type Material%20Object%20Reference))
  (bind _cylinder (Variables|Default|GetCylinder))
  (Components|StaticMesh|SetStaticMesh _cylinder DButtonMesh)
  (Rendering|Material|SetMaterial _cylinder 0 DButtonMat))

(fn ChangeScale)