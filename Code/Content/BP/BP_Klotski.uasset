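; BP_Klotski is a sliding-tile puzzle manager for eight buttons on a 3x3 grid with one empty cell.
; On BeginPlay it spawns BP_KlotskiButton actors, assigning each a grid coordinate, a parent reference and its array index.
; MoveButton finds the unoccupied cell and moves the chosen button there if their linear indices differ by 1 or 3.
; That index-only adjacency test also accepts moves that wrap between rows.
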(event EventBeginPlay
  (bind _buttons (Variables|Components|GetButtons))
  ;[1 1 1] Construct Buttons
  (for _index (range 0 7)
    (Development|PrintString (Utilities|String|ToString(Integer) _index))
    (bind _returnvalue (Game|SpawnActorfromClass "/Game/BP/BP_KlotskiButton.BP_KlotskiButton_C" (Math|Transform|MakeTransform "0, 0, 0") "Undefined" 0 0))
    (bind _returnvalue_2 (Utilities|Array|Add _buttons _returnvalue))
    (Default|SetCoord (Utilities|Array|Get(acopy) _buttons _returnvalue_2) (Utilities|NumtoCoord _index))
    (Variables|/Game/BP/BP_KlotskiButton.BP_KlotskiButton_C|SetParent (Utilities|Array|Get(acopy) _buttons _returnvalue_2) (Utilities|ResolveSoftReference self))
    (Variables|/Game/BP/BP_KlotskiButton.BP_KlotskiButton_C|SetIndexInParent (Utilities|Array|Get(acopy) _buttons _returnvalue_2) _returnvalue_2)))

(event Collision|EventActorBeginOverlap
  (params (OtherActor :type Actor%20Object%20Reference)))

(event EventTick
  (params (DeltaSeconds :type Float%20%28single-precision%29)))

(fn ConstructionScript)

(fn MoveButton
  (params (ButtonIndex :type Integer))
  (bind _buttons (Variables|Components|GetButtons))
  (bind _hasbutton (LocalVariables|GethasButton))
  (bind _output (Utilities|Array|Get(acopy) _buttons ButtonIndex))
  (for _array_element (Variables|Components|GetButtons)
    (Utilities|Array|SetArrayElem _hasbutton (Utilities|CoordtoNum (Variables|/Game/BP/BP_KlotskiButton.BP_KlotskiButton_C|GetCoord _array_element)) true))
  (for (_array_element_2 _array_index) _hasbutton
    (if (Math|Boolean|Equal(Boolean) _array_element_2 false)
      (LocalVariables|SetemptyCoord (Utilities|NumtoCoord _array_index))))
  (if (Math|Boolean|ORBoolean (== (- (Utilities|CoordtoNum (Variables|/Game/BP/BP_KlotskiButton.BP_KlotskiButton_C|GetCoord _output)) (Utilities|CoordtoNum (LocalVariables|GetemptyCoord))) 1) (== (- (Utilities|CoordtoNum (Variables|/Game/BP/BP_KlotskiButton.BP_KlotskiButton_C|GetCoord _output)) (Utilities|CoordtoNum (LocalVariables|GetemptyCoord))) -1) (== (- (Utilities|CoordtoNum (Variables|/Game/BP/BP_KlotskiButton.BP_KlotskiButton_C|GetCoord _output)) (Utilities|CoordtoNum (LocalVariables|GetemptyCoord))) 3) (== (- (Utilities|CoordtoNum (Variables|/Game/BP/BP_KlotskiButton.BP_KlotskiButton_C|GetCoord _output)) (Utilities|CoordtoNum (LocalVariables|GetemptyCoord))) -3)) ; check whether valid
    (Default|SetCoord _output (LocalVariables|GetemptyCoord))))