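; BP_Room12_ControllerLine is a line piece, apparently for a Room 12 controller, that spans two Y offsets and can change material.
; SetPos moves the Trans component to the midpoint of the offsets and scales its Y by their distance over 100, keeping fixed X and Z scale.
; SetMat swaps the material on the Ring component.
; It has no active event logic, so it relies on external calls to these functions.
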(event EventBeginPlay)

(event Collision|EventActorBeginOverlap
  (params (OtherActor :type Actor%20Object%20Reference)))

(event EventTick
  (params (DeltaSeconds :type Float%20%28single-precision%29)))

(fn ConstructionScript)

(fn SetPos
  (params (OffsetA :type Float%20%28single-precision%29) (OffsetB :type Float%20%28single-precision%29))
  (bind _trans (Variables|Default|GetTrans))
  (bind _relativelocation (Variables|/Script/Engine.SceneComponent|GetRelativeLocation _trans))
  (bind (_x _y _z) (Math|Vector|BreakVector _relativelocation))
  (Transformation|SetRelativeLocation _trans (Math|Vector|MakeVector _x (* (+ OffsetA OffsetB) 0.5) _z) false false)
  (Transformation|SetRelativeScale3D _trans (Math|Vector|MakeVector 4.0 (/ (Math|Float|Absolute(Float) (- OffsetB OffsetA)) 1e+02) 1.0)))

(fn SetMat
  (params (Mat :type Material%20Object%20Reference))
  (Rendering|Material|SetMaterial (Variables|Default|GetRing) 0 Mat))