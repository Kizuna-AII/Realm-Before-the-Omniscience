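; Keypad puzzle lock whose buttons toggle between O and X until their combined string matches the password.
; AddButton spawns a centered row of BP_KeypadButton_OX actors, each linked back by parent and index, with non-changeable ones prefilled from the password.
; ChangeNumber flips a button while locked, then compares the concatenated input to the password, unlocking and firing OnUnlocked on a match.
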(fn ConstructionScript)

(fn ChangeNumber
  (params (Index :type Integer))
  (bind _changeable (Variables|组件|GetChangeable))
  (bind _buttons (Variables|Components|GetButtons))
  (bind _output (Utilities|Array|Get(acopy) _buttons Index))
  (bind _output_2 (Utilities|Array|Get(acopy) _changeable Index))
  (if (Variables|Components|GetisLocked)
    (switch string (Variables|/Game/BP/BP_KeypadButton_OX.BP_KeypadButton_OX_C|GetNumber _output)
      (:O
        (Default|SetNumber _output "X" _output_2))
      (:X
        (Default|SetNumber _output "O" _output_2)))
    (bind _password (CallFunction|GetInputPassword))
    (if (Utilities|Enum|Equal(Enum) _password (Variables|Components|GetPassword))
      (Variables|Components|SetisLocked false)
      (Default|CallOnUnlocked))))

(fn GetInputPassword
  (for _array_element (Variables|Components|GetButtons)
    (LocalVariables|SetRes (Utilities|String|Append (LocalVariables|GetRes) (Variables|/Game/BP/BP_KeypadButton_OX.BP_KeypadButton_OX_C|GetNumber _array_element))))
  (return (LocalVariables|GetRes)))

(fn AddButton
  (params (NumOfDigits :type Integer))
  (bind _returnvalue (- NumOfDigits 1))
  (bind _buttons (Variables|Components|GetButtons))
  ;[1 1 1] Construct Buttons
  (for _index (range 0 _returnvalue)
    (bind _returnvalue_2 (Game|SpawnActorfromClass "/Game/BP/BP_KeypadButton_OX.BP_KeypadButton_OX_C" (Math|Transform|MakeTransform "0, 0, 0") "Undefined" 0 0))
    (bind _returnvalue_3 (Utilities|Array|Add _buttons _returnvalue_2))
    (Variables|/Game/BP/BP_KeypadButton_OX.BP_KeypadButton_OX_C|SetParent (Utilities|Array|Get(acopy) _buttons _returnvalue_3) self)
    (Variables|/Game/BP/BP_KeypadButton_OX.BP_KeypadButton_OX_C|SetIndexInParent (Utilities|Array|Get(acopy) _buttons _returnvalue_3) _returnvalue_3)
    (Default|SetChangeable (Utilities|Array|Get(acopy) _buttons _returnvalue_3) (Utilities|Array|Get(acopy) (Variables|组件|GetChangeable) _returnvalue_3))
    (if (Utilities|Array|Get(acopy) (Variables|组件|GetChangeable) _returnvalue_3)
      (Default|SetNumber (Utilities|Array|Get(acopy) _buttons _returnvalue_3) "O" (Utilities|Array|Get(acopy) (Variables|组件|GetChangeable) _returnvalue_3))
      (else
        (Default|SetNumber (Utilities|Array|Get(acopy) _buttons _returnvalue_3) (Utilities|String|GetSubstring (Variables|Components|GetPassword) _returnvalue_3) (Utilities|Array|Get(acopy) (Variables|组件|GetChangeable) _returnvalue_3))))
    (Default|SetCoord (Utilities|Array|Get(acopy) _buttons _returnvalue_3) (Math|Vector2D|MakeVector2D (- (Math|Conversions|ToFloat(Integer) _returnvalue_3) (/ (Math|Conversions|ToFloat(Integer) _returnvalue) 2.0)) 0.0))))