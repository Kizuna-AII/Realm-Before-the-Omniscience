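; BP_KlotskiButton is a clickable numbered tile in a Klotski sliding puzzle, showing its digit (0–9) through the Cube's material.
; A click passes the tile's index to the parent's MoveButton.
; SetCoord fires the OnSetCoord dispatcher, which plays a timeline that lerps between old and target positions.
; Each timeline update transforms that position by the parent's transform and copies the parent's rotation and scale.
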(event Custom|OnSetCoord_Event
  (params (TargetCoord :type Vector) (OldCoord :type Vector))
  (bind _parent (Variables|Components|GetParent))
  (bind _output (Utilities|ResolveSoftReference _parent))
  ;[1 1 1] Process SetCoord Timeline Effect
  (bind _newtrack_0 (Timeline|ButtonMoveTimeline PlayFromStart)
    (:Update
      (Transformation|SetActorLocationAndRotation (Math|Conversions|ToVector(Vector4) (Class|KismetMathLibrary|TransformVector4 (Math|Transform|ToMatrix(Transform) (Transformation|GetActorTransform _output)) (Math|Vector4|MakeVector4 (.X (Math|Vector|BreakVector (Math|Vector|Lerp(Vector) OldCoord TargetCoord _newtrack_0))) (.Y (Math|Vector|BreakVector (Math|Vector|Lerp(Vector) OldCoord TargetCoord _newtrack_0))) (.Z (Math|Vector|BreakVector (Math|Vector|Lerp(Vector) OldCoord TargetCoord _newtrack_0))) 1.0))) (Transformation|GetActorRotation _output))
      (Transformation|SetActorScale3D (Transformation|GetActorScale3D _output)))))

(event EventBeginPlay
  ;[1 1 1] Process SetCoord Timeline Effect
  (EventDispatchers|BindEventtoOnSetCoord (delegate Custom|OnSetCoord_Event)))

(event EventOnMouseClicked
  (Development|PrintString "Clicked")
  (Default|MoveButton (Utilities|ResolveSoftReference (Variables|Components|GetParent)) (Variables|Components|GetIndexInParent)))

(fn ConstructionScript)

(fn SetCoord
  (params (Coord :type Vector%202D%20Structure))
  (bind _output_get (LocalVariables|SetOldCoord (Variables|Components|GetCoord)))
  (bind _output_get_2 (Variables|Components|SetCoord Coord))
  (Default|CallOnSetCoord (Utilities|ConvertRealCoord _output_get_2) (Utilities|ConvertRealCoord _output_get)))

(fn SetNumber
  (params (Number :type Integer))
  (bind _cube (Variables|Default|GetCube))
  (bind _output_get (Variables|Components|SetNumber Number))
  (switch int _output_get
    (:0
      (Rendering|Material|SetMaterial _cube 0 "/Game/Material/Number/0_Mat_NT.0_Mat_NT"))
    (:1
      (Rendering|Material|SetMaterial _cube 0 "/Game/Material/Number/1_Mat_NT.1_Mat_NT"))
    (:2
      (Rendering|Material|SetMaterial _cube 0 "/Game/Material/Number/2_Mat_NT.2_Mat_NT"))
    (:3
      (Rendering|Material|SetMaterial _cube 0 "/Game/Material/Number/3_Mat_NT.3_Mat_NT"))
    (:4
      (Rendering|Material|SetMaterial _cube 0 "/Game/Material/Number/4_Mat_NT.4_Mat_NT"))
    (:5
      (Rendering|Material|SetMaterial _cube 0 "/Game/Material/Number/5_Mat_NT.5_Mat_NT"))
    (:6
      (Rendering|Material|SetMaterial _cube 0 "/Game/Material/Number/6_Mat_NT.6_Mat_NT"))
    (:7
      (Rendering|Material|SetMaterial _cube 0 "/Game/Material/Number/7_Mat_NT.7_Mat_NT"))
    (:8
      (Rendering|Material|SetMaterial _cube 0 "/Game/Material/Number/8_Mat_NT.8_Mat_NT"))
    (:9
      (Rendering|Material|SetMaterial _cube 0 "/Game/Material/Number/9_Mat_NT.9_Mat_NT"))))