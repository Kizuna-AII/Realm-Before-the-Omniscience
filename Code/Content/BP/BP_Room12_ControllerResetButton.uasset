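; BP_Room12_ControllerResetButton is a clickable button that resets the Room 12 controller.
; Hover toggles a custom-depth highlight on the button mesh, and a click casts the owner to BP_Room12_Controller, calls Reset and prints a debug string.
; Tick polls the current language every frame and swaps the button material between Chinese and English versions, defaulting to English.
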(event EventOnMouseUnfover
  (Rendering|SetRenderCustomDepth (Variables|Default|GetButton) false))

(event EventTick
  (params (DeltaSeconds :type Float%20%28single-precision%29))
  (bind _button (Variables|Default|GetButton))
  (switch string (Utilities|String|GetSubstring (Class|KismetInternationalizationLibrary|GetCurrentLanguage) 0 2)
    (:Default
      (Rendering|Material|SetMaterial _button 0 "/Game/Material/RESET_en_Mat.RESET_en_Mat" :!label _label))
    (:zh
      (Rendering|Material|SetMaterial _button 0 "/Game/Material/Reset_cn_Mat.Reset_cn_Mat"))
    (:en
      (goto _label))))

(event EventOnMouseFover
  (Rendering|SetRenderCustomDepth (Variables|Default|GetButton) true))

(event EventOnMouseClicked
  (bind _asbp_room_12_controller (Utilities|Casting|CastToBP_Room12_Controller (Components|GetOwner)))
  (Default|Reset _asbp_room_12_controller)
  (Development|PrintString "ABC"))

(fn ConstructionScript
  (|CallParentFunction))