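; Room 6 puzzle screen: a 5x5 sliding-block board that spawns fixed columns, single-cell buttons and two-cell buttons at BeginPlay.
; I/J/K/L keys move the selected button after rebuilding free cells and valid directions.
; Columns block only single buttons, and double buttons slide only along their long axis.
; A linked child screen has its buttons made unselectable and mirrors the parent's moves without validation, playing a sound.
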(event EventBeginPlay
  (CallFunction|AddColumn "(X=1.000000,Y=1.000000)")
  (CallFunction|AddColumn "(X=3.000000,Y=1.000000)" 1)
  (CallFunction|AddColumn "(X=1.000000,Y=3.000000)" 3)
  (CallFunction|AddColumn "(X=3.000000,Y=3.000000)" 2)
  (CallFunction|AddSingleButton "(X=4.000000,Y=0.000000)")
  (CallFunction|AddSingleButton "(X=0.000000,Y=1.000000)")
  (CallFunction|AddSingleButton "(X=1.000000,Y=2.000000)")
  (CallFunction|AddSingleButton "(X=3.000000,Y=2.000000)")
  (CallFunction|AddDoubleButton)
  (CallFunction|AddDoubleButton "(X=2.000000,Y=0.000000)")
  (CallFunction|AddDoubleButton "(X=0.000000,Y=2.000000)" 1)
  (CallFunction|AddDoubleButton "(X=2.000000,Y=2.000000)" 1)
  (CallFunction|AddDoubleButton "(X=0.000000,Y=4.000000)")
  (CallFunction|AddDoubleButton "(X=2.000000,Y=4.000000)"))

(event Input|KeyboardEvents|J
  (params (Key :type Key%20Structure))
  (:Pressed
    (CallFunction|MoveSingleButton (Variables|Components|GetSingleButtonSelected) 3)
    (CallFunction|MoveDoubleButton (Variables|Components|GetDoubleButtonSelected) 3)))

(event Input|KeyboardEvents|K
  (params (Key :type Key%20Structure))
  (:Pressed
    (CallFunction|MoveSingleButton (Variables|Components|GetSingleButtonSelected) 2)
    (CallFunction|MoveDoubleButton (Variables|Components|GetDoubleButtonSelected) 2)))

(event Input|KeyboardEvents|L
  (params (Key :type Key%20Structure))
  (:Pressed
    (CallFunction|MoveSingleButton (Variables|Components|GetSingleButtonSelected) 1)
    (CallFunction|MoveDoubleButton (Variables|Components|GetDoubleButtonSelected) 1)))

(event Input|KeyboardEvents|I
  (params (Key :type Key%20Structure))
  (:Pressed
    (CallFunction|MoveSingleButton (Variables|Components|GetSingleButtonSelected))
    (CallFunction|MoveDoubleButton (Variables|Components|GetDoubleButtonSelected))))

(fn ConstructionScript)

(fn AddColumn
  (params (XZ :type Vector%202D%20Structure) (Direction :type Integer))
  (bind _returnvalue (Game|SpawnActorfromClass "/Game/BP/BP_Room6_Column.BP_Room6_Column_C" (Math|Transform|MakeTransform "0, 0, 0") "Undefined" 0 0))
  (Default|ChangeMesh _returnvalue (Variables|组件|GetColumnMesh) (Variables|组件|GetColumnMat))
  (Variables|/Game/BP/BP_Room6_Column.BP_Room6_Column_C|SetScale _returnvalue (Variables|组件|GetColumnScale))
  (Utilities|Array|Add (Variables|Components|GetColumns) _returnvalue)
  (Variables|/Game/BP/BP_Room6_Column.BP_Room6_Column_C|SetParent _returnvalue (Utilities|ResolveSoftReference self))
  (Variables|/Game/BP/BP_Room6_Column.BP_Room6_Column_C|SetDirection _returnvalue Direction)
  (Default|SetCoord _returnvalue XZ)
  (Collision|SetActorEnableCollision _returnvalue true))

(fn MoveSingleButton
  (params (Index :type Integer) (Direction :type Integer))
  (bind _str (Utilities|DirectiontoStr Direction))
  (bind _singlebuttons (Variables|Components|GetSingleButtons))
  (bind _childscreen (Variables|Components|GetChildScreen))
  (bind _output (Utilities|Array|Get(acopy) _singlebuttons Index))
  (bind _coord (Variables|/Game/BP/BP_Room6_Button_Single.BP_Room6_Button_Single_C|GetCoord _output))
  ;[1 1 1] Move Child Button if existed
  (if (== (Variables|Components|GetState) 1)
    (bind _validdirectionres (CallFunction|GetSingleButtonValidDirection _coord))
    (if (Utilities|Set|Contains _validdirectionres Direction) ; check whether valid
      (Default|SetCoord _output (Utilities|CoordAfterMove _coord Direction))
      (if (== _childscreen 0)
        _
        (else
          (CallFunction|MoveSingleButtonWithoutCheck _childscreen Index Direction)))
      (Development|PrintString (Utilities|String|Append "Moved To: " _str))
      (else
        (Development|PrintString (Utilities|String|Append "Cannot Move To" _str))))))

(fn MoveDoubleButton
  (params (Index :type Integer) (Direction :type Integer))
  (bind _str (Utilities|DirectiontoStr Direction))
  (bind _childscreen (Variables|Components|GetChildScreen))
  (bind _doublebuttons (Variables|Components|GetDoubleButtons))
  (bind _output (Utilities|Array|Get(acopy) _doublebuttons Index))
  (if (== (Variables|Components|GetState) 2)
    (bind _validdirectionres (CallFunction|GetDoubleButtonValidDirection Index))
    (if (Utilities|Set|Contains _validdirectionres Direction) ; check whether valid
      (Default|SetCoord _output (Utilities|CoordAfterMove (Variables|/Game/BP/BP_Room6_Button_Double.BP_Room6_Button_Double_C|GetCoord _output) Direction))
      (if (== _childscreen 0)
        _
        (else
          (CallFunction|MoveDoubleButtonWithoutCheck _childscreen Index Direction)))
      (Development|PrintString (Utilities|String|Append "Moved To: " _str))
      (else
        (Development|PrintString (Utilities|String|Append "Cannot Move To" _str))))))

(fn GetSingleButtonValidDirection
  (params (Coord :type Vector%202D%20Structure))
  (bind _validdirection (LocalVariables|GetValidDirection))
  (LocalVariables|SetTargetCoord Coord)
  (LocalVariables|SetTargetPos (Utilities|CoordtoNum Coord))
  ;[1 1 1] Generate initial value for ValidPos
  (for _index (range 0 24)
    (Utilities|Set|Add (LocalVariables|GetValidPos) _index))
  ;[1 1 1] Compute ValidPos
  (for _array_element (Variables|Components|GetSingleButtons)
    (Utilities|Set|Remove (LocalVariables|GetValidPos) (Utilities|CoordtoNum (Variables|/Game/BP/BP_Room6_Button_Single.BP_Room6_Button_Single_C|GetCoord _array_element))))
  ;[1 1 1] Compute ValidDiretion
  (for _index_2 (range 0 3)
    (Utilities|Set|Add (LocalVariables|GetValidDirection) _index_2))
  (for (_array_element_2 _array_index) (Variables|Components|GetColumns)
    (Utilities|Set|Remove (LocalVariables|GetValidPos) (Utilities|CoordtoNum (Variables|/Game/BP/BP_Room6_Column.BP_Room6_Column_C|GetCoord _array_element_2))))
  (for _array_element_3 (Variables|Components|GetDoubleButtons)
    (Utilities|Set|Remove (LocalVariables|GetValidPos) (Utilities|CoordtoNum (Variables|/Game/BP/BP_Room6_Button_Double.BP_Room6_Button_Double_C|GetCoord _array_element_3)))
    (Utilities|Set|Remove (LocalVariables|GetValidPos) (Utilities|CoordtoNum (+ (Variables|/Game/BP/BP_Room6_Button_Double.BP_Room6_Button_Double_C|GetCoord _array_element_3) (Utilities|Select :Index (Variables|/Game/BP/BP_Room6_Button_Double.BP_Room6_Button_Double_C|GetExpandDir _array_element_3) :Option%200 "(X=1.000000,Y=0.000000)" :Option%201 "(X=0.000000,Y=1.000000)")))))
  (if (== (Math|Integer|%(Integer) (LocalVariables|GetTargetPos) 5) 0) ; x = 0
    (Utilities|Set|Remove (LocalVariables|GetValidDirection) 1))
  (if (== (Math|Integer|%(Integer) (LocalVariables|GetTargetPos) 5) 4) ; x = 4
    (Utilities|Set|Remove (LocalVariables|GetValidDirection) 3))
  (if (== (/ (LocalVariables|GetTargetPos) 5) 0) ; y = 0
    (Utilities|Set|Remove (LocalVariables|GetValidDirection) 2))
  (if (== (/ (LocalVariables|GetTargetPos) 5) 4) ; y = 4
    (Utilities|Set|Remove (LocalVariables|GetValidDirection) 0))
  ;[1 1 1] Compute Final Set
  (bind _result (Utilities|Set|ToArray (LocalVariables|GetValidDirection)))
  (for _array_element_4 _result
    (if (not (Utilities|Set|Contains (LocalVariables|GetValidPos) (Utilities|CoordtoNum (Utilities|CoordAfterMove (LocalVariables|GetTargetCoord) _array_element_4)))) ; check whether valid
      (Utilities|Set|Remove _validdirection _array_element_4)))
  (bind _result_2 (Utilities|Set|ToArray _validdirection))
  ;[1 1 1] Debug Info
  (LocalVariables|SetTempStr (Utilities|String|Append "State: " (Utilities|String|ToString(Integer) (Variables|Components|GetState)) "Valid Dir: "))
  (for _array_element_5 _result_2
    (LocalVariables|SetTempStr (Utilities|String|Append (LocalVariables|GetTempStr) (Utilities|DirectiontoStr _array_element_5) ",")))
  (Development|PrintString (LocalVariables|GetTempStr))
  (return _validdirection))

(fn GetDoubleButtonValidDirection
  (params (Index :type Integer))
  (bind _doublebuttons (Variables|Components|GetDoubleButtons))
  (bind _validdirection (LocalVariables|GetValidDirection))
  (bind _output (Utilities|Array|Get(acopy) _doublebuttons Index))
  (bind _coord (Variables|/Game/BP/BP_Room6_Button_Double.BP_Room6_Button_Double_C|GetCoord _output))
  (LocalVariables|SetTargetButton _output)
  (LocalVariables|SetTargetCoord _coord)
  (LocalVariables|SetTargetPos (Utilities|CoordtoNum _coord))
  ;[1 1 1] Generate initial value for ValidPos
  (for _index (range 0 24)
    (Utilities|Set|Add (LocalVariables|GetValidPos) _index))
  ;[1 1 1] Compute ValidPos
  (for _array_element (Variables|Components|GetSingleButtons)
    (Utilities|Set|Remove (LocalVariables|GetValidPos) (Utilities|CoordtoNum (Variables|/Game/BP/BP_Room6_Button_Single.BP_Room6_Button_Single_C|GetCoord _array_element))))
  (for _array_element_2 (Variables|Components|GetDoubleButtons)
    (Utilities|Set|Remove (LocalVariables|GetValidPos) (Utilities|CoordtoNum (Variables|/Game/BP/BP_Room6_Button_Double.BP_Room6_Button_Double_C|GetCoord _array_element_2)))
    (Utilities|Set|Remove (LocalVariables|GetValidPos) (Utilities|CoordtoNum (+ (Variables|/Game/BP/BP_Room6_Button_Double.BP_Room6_Button_Double_C|GetCoord _array_element_2) (Utilities|Select :Index (Variables|/Game/BP/BP_Room6_Button_Double.BP_Room6_Button_Double_C|GetExpandDir _array_element_2) :Option%200 "(X=1.000000,Y=0.000000)" :Option%201 "(X=0.000000,Y=1.000000)")))))
  ;[1 1 1] Compute ValidDiretion
  (switch int (Variables|/Game/BP/BP_Room6_Button_Double.BP_Room6_Button_Double_C|GetExpandDir (LocalVariables|GetTargetButton))
    (:0
      (if (and (<= (.X (Math|Vector2D|BreakVector2D (+ (LocalVariables|GetTargetCoord) "(X=2.000000,Y=0.000000)"))) 4.0) (Utilities|Set|Contains (LocalVariables|GetValidPos) (Utilities|CoordtoNum (+ (LocalVariables|GetTargetCoord) "(X=2.000000,Y=0.000000)"))))
        (Utilities|Set|Add (LocalVariables|GetValidDirection) 3))
      (if (and (>= (.X (Math|Vector2D|BreakVector2D (+ (LocalVariables|GetTargetCoord) "(X=-1.000000,Y=0.000000)"))) 0.0) (Utilities|Set|Contains (LocalVariables|GetValidPos) (Utilities|CoordtoNum (+ (LocalVariables|GetTargetCoord) "(X=-1.000000,Y=0.000000)"))))
        (Utilities|Set|Add (LocalVariables|GetValidDirection) 1)))
    (:1
      (if (Utilities|Set|Contains (LocalVariables|GetValidPos) (Utilities|CoordtoNum (+ (LocalVariables|GetTargetCoord) "(X=0.000000,Y=2.000000)")))
        (Utilities|Set|Add (LocalVariables|GetValidDirection) 0))
      (if (Utilities|Set|Contains (LocalVariables|GetValidPos) (Utilities|CoordtoNum (+ (LocalVariables|GetTargetCoord) "(X=0.000000,Y=-1.000000)")))
        (Utilities|Set|Add _validdirection 2))))
  ;[1 1 1] Debug Info
  (LocalVariables|SetTempStr "Valid Dir: ")
  (bind _result (Utilities|Set|ToArray (LocalVariables|GetValidDirection)))
  (for _array_element_3 _result
    (LocalVariables|SetTempStr (Utilities|String|Append (LocalVariables|GetTempStr) (Utilities|DirectiontoStr _array_element_3) ",")))
  (if (Utilities|Enum|Equal(Enum) (LocalVariables|GetTempStr) "")
    (Development|PrintString "Cannot Move")
    (else
      (Development|PrintString (LocalVariables|GetTempStr))))
  (return _validdirection))

(fn AddSingleButton
  (params (XZ :type Vector%202D%20Structure))
  (bind _returnvalue (Game|SpawnActorfromClass "/Game/BP/BP_Room6_Button_Single.BP_Room6_Button_Single_C" (Math|Transform|MakeTransform "0, 0, 0") "Undefined" 0 0))
  (Default|ChangeMesh _returnvalue (Variables|组件|GetButtonMesh) (Variables|组件|GetButtonMat))
  (Variables|/Game/BP/BP_Room6_Button_Single.BP_Room6_Button_Single_C|SetScale _returnvalue (Variables|组件|GetButtonScale))
  (bind _returnvalue_2 (Utilities|Array|Add (Variables|Components|GetSingleButtons) _returnvalue))
  (Variables|/Game/BP/BP_Room6_Button_Single.BP_Room6_Button_Single_C|SetParent _returnvalue (Utilities|ResolveSoftReference self))
  (Variables|/Game/BP/BP_Room6_Button_Single.BP_Room6_Button_Single_C|SetIndexInParent _returnvalue _returnvalue_2)
  (Default|SetCoord _returnvalue XZ))

(fn AddDoubleButton
  (params (XZ :type Vector%202D%20Structure) (ExpandDir :type Integer))
  (bind _returnvalue (Game|SpawnActorfromClass "/Game/BP/BP_Room6_Button_Double.BP_Room6_Button_Double_C" (Math|Transform|MakeTransform "0, 0, 0") "Undefined" 0 0 0 0 0))
  (Default|ChangeMesh _returnvalue (Variables|组件|GetDButtonMesh) (Variables|组件|GetDButtonMat))
  (Variables|/Game/BP/BP_Room6_Button_Double.BP_Room6_Button_Double_C|SetScale _returnvalue (Variables|组件|GetDButtonScale))
  (bind _returnvalue_2 (Utilities|Array|Add (Variables|Components|GetDoubleButtons) _returnvalue))
  (Variables|/Game/BP/BP_Room6_Button_Double.BP_Room6_Button_Double_C|SetParent _returnvalue (Utilities|ResolveSoftReference self))
  (Variables|/Game/BP/BP_Room6_Button_Double.BP_Room6_Button_Double_C|SetIndexInParent _returnvalue _returnvalue_2)
  (Variables|/Game/BP/BP_Room6_Button_Double.BP_Room6_Button_Double_C|SetExpandDir _returnvalue ExpandDir)
  (Default|SetCoord _returnvalue XZ))

(fn SelectSingleButton
  (params (Index :type Integer))
  (bind _output_get (Variables|Components|SetSingleButtonSelected Index))
  (Variables|Components|SetState 1)
  (Development|PrintString (Utilities|String|Append "Select:  id = " (Utilities|String|ToString(Integer) _output_get) ", Coord = " (Utilities|String|ToString(Vector2d) (Variables|/Game/BP/BP_Room6_Button_Single.BP_Room6_Button_Single_C|GetCoord (Utilities|Array|Get(acopy) (Variables|Components|GetSingleButtons) _output_get))))))

(fn SelectDoubleButton
  (params (Index :type Integer))
  (bind _output_get (Variables|Components|SetDoubleButtonSelected Index))
  (Variables|Components|SetState 2)
  (Development|PrintString (Utilities|String|Append "Select:  id = " (Utilities|String|ToString(Integer) _output_get) ", Coord= " (Utilities|String|ToString(Vector2d) (Variables|/Game/BP/BP_Room6_Button_Double.BP_Room6_Button_Double_C|GetCoord (Utilities|Array|Get(acopy) (Variables|Components|GetDoubleButtons) _output_get))) ", Dir = " (Utilities|String|ToString(Integer) (Variables|/Game/BP/BP_Room6_Button_Double.BP_Room6_Button_Double_C|GetExpandDir (Utilities|Array|Get(acopy) (Variables|Components|GetDoubleButtons) _output_get))))))

(fn UnselectSingleButton
  (params (Index :type Integer))
  (if (and (== (Variables|Components|GetState) 1) (== Index (Variables|Components|GetSingleButtonSelected)))
    (Variables|Components|SetState 0)
    (Development|PrintString "Unselect!")))

(fn UnselectDoubleButton
  (params (Index :type Integer))
  (if (and (== (Variables|Components|GetState) 2) (== (Variables|Components|GetDoubleButtonSelected) Index))
    (Variables|Components|SetState 0)
    (Development|PrintString "Unselect!")))

(fn SetParentScreen
  (params (ParentScreen :type BP%20Room%206%20Screen%20Object%20Reference))
  (Variables|BP_Room6_Screen_C|SetChildScreen ParentScreen self)
  (Variables|Components|SetParentScreen ParentScreen)
  (for _array_element (Variables|Components|GetSingleButtons)
    (Variables|/Game/BP/BP_Room6_Button_Single.BP_Room6_Button_Single_C|SetSelectable _array_element false))
  (for _array_element_2 (Variables|Components|GetDoubleButtons)
    (Variables|/Game/BP/BP_Room6_Button_Double.BP_Room6_Button_Double_C|SetSelectable _array_element_2 false)))

(fn MoveSingleButtonWithoutCheck
  (params (Index :type Integer) (Direction :type Integer))
  (bind _singlebuttons (Variables|Components|GetSingleButtons))
  (bind _output (Utilities|Array|Get(acopy) _singlebuttons Index))
  (Default|SetCoord _output (Utilities|CoordAfterMove (Variables|/Game/BP/BP_Room6_Button_Single.BP_Room6_Button_Single_C|GetCoord _output) Direction))
  (CallFunction|PlayFractionSE))

(fn MoveDoubleButtonWithoutCheck
  (params (Index :type Integer) (Direction :type Integer))
  (bind _doublebuttons (Variables|Components|GetDoubleButtons))
  (bind _output (Utilities|Array|Get(acopy) _doublebuttons Index))
  (Default|SetCoord _output (Utilities|CoordAfterMove (Variables|/Game/BP/BP_Room6_Button_Double.BP_Room6_Button_Double_C|GetCoord _output) Direction))
  (CallFunction|PlayFractionSE))

(fn PlayFractionSE
  (if (Variables|组件|GetisPosition)
    (Audio|SpawnSoundatLocation "/Game/Audio/FractionSE_Cue.FractionSE_Cue" (Variables|组件|GetSoundPosition) "0, 0, 0" 1.0 1.0 0.0 0 0)
    (else
      (Audio|SpawnSound2D "/Game/Audio/FractionSE_Cue.FractionSE_Cue" 1.0 1.0 0.0 0))))