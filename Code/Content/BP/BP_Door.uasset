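; BP_Door is a swinging door that other logic can open and close through its OpenDoor and CloseDoor functions.
; Both functions set the IsOpen flag, toggle collision for the whole actor (off when open) and print a debug message.
; Tick polls IsOpen every frame to play or reverse Timeline_OpenDoor, whose Angle track drives the relative yaw of DoorBody.
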(event EventTick
  (params (DeltaSeconds :type Float%20%28single-precision%29))
  (if (Variables|Default|GetisOpen)
    (bind _angle (Timeline|Timeline_OpenDoor Play)
      (:Update
        (Transformation|SetRelativeRotation (Variables|Default|GetDoorBody) (Math|Rotator|MakeRotator 0.0 0.0 _angle) false false)))
    (else
      (Timeline|Timeline_OpenDoor Reverse))))

(fn ConstructionScript)

(fn OpenDoor
  (Collision|SetActorEnableCollision (Components|GetOwner (Variables|Default|GetDoorBody)) false)
  (Development|PrintString "Open Door")
  (Variables|Default|SetisOpen true))

(fn CloseDoor
  (Collision|SetActorEnableCollision (Components|GetOwner (Variables|Default|GetDoorBody)) true)
  (Development|PrintString "Close Door")
  (Variables|Default|SetisOpen false))