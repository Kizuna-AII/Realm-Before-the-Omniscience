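; A clickable button for the Room 12 controller that highlights on hover and reports clicks to that controller.
; Hover and unhover events toggle custom depth rendering on the Button component.
; On click, it casts its owner to BP_Room12_Controller and passes itself to TryToSelect, leaving selection logic to the controller.
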(event EventOnMouseUnfover
  (Rendering|SetRenderCustomDepth (Variables|Default|GetButton) false))

(event EventOnMouseFover
  (Rendering|SetRenderCustomDepth (Variables|Default|GetButton) true))

(event EventOnMouseClicked
  (bind _asbp_controller (Utilities|Casting|CastToBP_Room12_Controller (Components|GetOwner)))
  (Default|TrytoSelect _asbp_controller self))

(fn ConstructionScript
  (|CallParentFunction))