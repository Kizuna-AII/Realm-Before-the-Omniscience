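; Fire hazard actor for the Room 10 tunnel that respawns the player through its Parent when its capsule overlaps them.
; SetPos places it on a horizontal circle around Center, facing along the tangent with a roll spin, and offsets the fire mesh sideways.
; SetThick stretches the fire mesh to an angle-based arc length and a target cross-section.
; Nothing in this graph calls either function.
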(event OnComponentBeginOverlap(Capsule)
  (params (OverlappedComponent :type Primitive%20Component%20Object%20Reference) (OtherActor :type Actor%20Object%20Reference) (OtherComp :type Primitive%20Component%20Object%20Reference) (OtherBodyIndex :type Integer) (bFromSweep :type Boolean) (SweepResult :type Hit%20Result%20Structure%20%28by%20ref%29))
  (if (== OtherActor (Game|GetPlayerCharacter 0))
    (Development|PrintString "Hot")
    (Default|PlayerRespawn (Variables|Components|GetParent))))

(fn ConstructionScript)

(fn SetPos
  (params (RadiusAngle :type Float%20%28single-precision%29) (SelfRotateAngle :type Float%20%28single-precision%29))
  (bind _p_fire (Variables|Default|GetP_Fire))
  (bind _relativelocation (Variables|/Script/Engine.SceneComponent|GetRelativeLocation _p_fire))
  (bind (_x _y _z) (Math|Vector|BreakVector _relativelocation))
  (Transformation|SetRelativeLocation (Variables|Default|GetP_Fire) (Math|Vector|MakeVector _x (* (Variables|Components|GetYOffset) 2.5e+02) _z) false false)
  (Transformation|SetActorLocationAndRotation (+ (Math|Conversions|ToVector(Vector2D) (* (Math|Vector2D|MakeVector2D (Math|Trig|Cos(Degrees) RadiusAngle) (Math|Trig|Sin(Degrees) RadiusAngle)) (Variables|Components|GetRadius))) (Variables|Components|GetCenter)) (Math|Rotator|CombineRotators (Math|Vector|RotatorfromAxisandAngle "1.000000,0.000000,0.000000" SelfRotateAngle) (Math|Vector|RotatorfromAxisandAngle "0,0.000000,1.000000" (+ RadiusAngle 9e+01)))))

(fn SetThick
  (params (Angle :type Float%20%28single-precision%29))
  (bind _meshsize (Variables|Components|GetMeshSize))
  (bind _targetsize (Variables|Components|GetTargetSize))
  (bind (_x _y _z) (Math|Vector|BreakVector _meshsize))
  (bind (_x_2 _y_2 _z_2) (Math|Vector|BreakVector _targetsize))
  (Transformation|SetWorldScale3D (Variables|Default|GetP_Fire) (Math|Vector|MakeVector (* (/ Angle 1.8e+02) (Math|Trig|GetPI) (+ (Variables|Components|GetRadius) (* _y_2 1.6125)) 1.0 (/ 1.0 _x)) (/ _y_2 _y) (/ _z_2 _z))))