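; Room 9 tunnel actor that builds a twisting tunnel along an arc and rolls it as the player jumps.
; BeginPlay spawns and attaches normal, special and outer pieces, narrowing boards on some segments; UpdateView positions each by arc angle and self-rotation plus a shared offset.
; Space triggers a jump and a timeline quarter-turn of that offset, while PlayerRespawn resets player and rotation.
; Holding I nudges rotation for testing; camera-driven rotation is disconnected.
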(event EventBeginPlay
  (bind _returnvalue (Math|Transform|MakeTransform "0, 0, 0"))
  ;[1 1 1] Construction
  (for _index (range 0 (- (Variables|Components|GetTotalPieceNum) 1))
    (bind _returnvalue_2 (Game|SpawnActorfromClass "/Game/BP/BP_Room9TunnelPiece.BP_Room9TunnelPiece_C" _returnvalue "Undefined" 0 0))
    (Utilities|Array|Add (Variables|Components|GetPieces) _returnvalue_2)
    (Transformation|AttachComponentToComponent _returnvalue_2 (Variables|Default|GetDefaultSceneRoot) "None" "KeepRelative" "KeepRelative" "KeepRelative" true))
  (for _index_2 (range 0 (- (Variables|Components|GetTotalSpecialPieceNum) 1))
    (bind _returnvalue_3 (Game|SpawnActorfromClass "/Game/BP/BP_Room9TunnelPiece.BP_Room9TunnelPiece_C" _returnvalue "Undefined" 0 0))
    (Utilities|Array|Add (Variables|Components|GetSpecialPieces) _returnvalue_3)
    (Transformation|AttachComponentToComponent _returnvalue_3 (Variables|Default|GetDefaultSceneRoot) "None" "KeepRelative" "KeepRelative" "KeepRelative" true))
  (for _index_3 (range 4 7)
    (Variables|/Game/BP/BP_Room9TunnelPiece.BP_Room9TunnelPiece_C|SetBoardLeftRatio (Utilities|Array|Get(acopy) (Variables|Components|GetPieces) _index_3) 0.33333))
  (for _index_4 (range 8 11)
    (Variables|/Game/BP/BP_Room9TunnelPiece.BP_Room9TunnelPiece_C|SetBoardRightRatio (Utilities|Array|Get(acopy) (Variables|Components|GetPieces) _index_4) 0.666667))
  (for _index_5 (range 12 14)
    (Variables|/Game/BP/BP_Room9TunnelPiece.BP_Room9TunnelPiece_C|SetBoardLeftRatio (Utilities|Array|Get(acopy) (Variables|Components|GetPieces) _index_5) 0.33333)
    (Variables|/Game/BP/BP_Room9TunnelPiece.BP_Room9TunnelPiece_C|SetBoardRightRatio (Utilities|Array|Get(acopy) (Variables|Components|GetPieces) _index_5) 0.666667))
  (for _index_6 (range 0 (- (Variables|Components|GetTotalOuterPieceNum) 1))
    (bind _returnvalue_4 (Game|SpawnActorfromClass "/Game/BP/BP_Room9TunnelOuterPiece.BP_Room9TunnelOuterPiece_C" (Math|Transform|MakeTransform "0, 0, 0") "Undefined" 0 0))
    (Utilities|Array|Add (Variables|Components|GetOuterPieces) _returnvalue_4)
    (Variables|/Game/BP/BP_Room9TunnelOuterPiece.BP_Room9TunnelOuterPiece_C|SetParent _returnvalue_4 self)
    (Transformation|AttachComponentToComponent _returnvalue_4 (Variables|Default|GetDefaultSceneRoot) "None" "KeepRelative" "KeepRelative" "KeepRelative" true))
  (CallFunction|UpdateView)
  (Utilities|FlowControl|Delay 0.5)
  (Variables|Components|SetSelfRotateOffsetAngle -1.8e+02)
  (CallFunction|UpdateView))

(event EventTick
  (params (DeltaSeconds :type Float%20%28single-precision%29))
  ;[1 1 1] Test
  (if (Game|Player|IsInputKeyDown (Game|GetPlayerController 0) "I")
    (Variables|Components|SetSelfRotateOffsetAngle (+ (Variables|Components|GetSelfRotateOffsetAngle) 1.0))
    (CallFunction|UpdateView)
    (Development|PrintString (Utilities|String|ToString(Float) (Variables|Components|GetSelfRotateOffsetAngle)))))

(event Input|KeyboardEvents|SpaceBar
  (params (Key :type Key%20Structure :default "None"))
  (bind _returnvalue (Game|GetPlayerCharacter 0))
  ;[1 1 1] Jump to Rotate
  (:Pressed
    (if (not (Variables|Components|GetisRotating))
      (if (== _returnvalue 0)
        _
        (else
          (Character|Jump _returnvalue)))
      (Development|PrintString "Jumped")
      (bind _newtrack_0 (Timeline|RotateTimeline PlayFromStart)
        (:Update
          (Variables|Components|SetisRotating true)
          (Variables|Components|SetSelfRotateOffsetAngle (+ (* _newtrack_0 -9e+01) (Variables|Components|GetSelfRotateOffsetAngleBase)))
          (CallFunction|UpdateView))
        (:Finished
          (Variables|Components|SetSelfRotateOffsetAngleBase (Variables|Components|GetSelfRotateOffsetAngle))
          (Variables|Components|SetisRotating false))))))

(fn ConstructionScript)

(fn UpdateView
  ;[1 1 1] Normal Pieces
  (for (_array_element _array_index) (Variables|Components|GetPieces)
    (Default|SetPos _array_element (Utilities|GetRadiusAngle (Math|Conversions|ToFloat(Integer) _array_index) (Variables|Components|GetTotalPieceNum)) (Utilities|GetSelfRotateAngle (Math|Conversions|ToFloat(Integer) _array_index)))
    (Default|SetThick _array_element (/ (Variables|Components|GetTotalRadiusAngle) (Math|Conversions|ToFloat(Integer) (Variables|Components|GetTotalPieceNum)))))
  ;[1 1 1] Special Pieces
  (for (_array_element_2 _array_index_2) (Variables|Components|GetSpecialPieces)
    (Default|SetPos _array_element_2 (Utilities|GetRadiusAngle (+ (* (Math|Conversions|ToFloat(Integer) _array_index_2) 0.666667) 6.0) (Variables|Components|GetTotalPieceNum)) (+ (* (Math|Conversions|ToFloat(Integer) _array_index_2) 9e+01) (Variables|Components|GetSelfRotateOffsetAngle)))
    (Default|SetThick _array_element_2 (/ (Variables|Components|GetTotalRadiusAngle) (Math|Conversions|ToFloat(Integer) (Variables|Components|GetTotalPieceNum)))))
  ;[1 1 1] Outer Pieces
  (for (_array_element_3 _array_index_3) (Variables|Components|GetOuterPieces)
    (Variables|/Game/BP/BP_Room9TunnelOuterPiece.BP_Room9TunnelOuterPiece_C|SetTargetSize _array_element_3 (Math|Vector|MakeVector 0.0 3e+03 3e+03))
    (Default|SetPos _array_element_3 (Utilities|GetRadiusAngle (Math|Conversions|ToFloat(Integer) _array_index_3) (Variables|Components|GetTotalOuterPieceNum)) (+ (Utilities|GetSelfRotateAngle 0.0) 2.0))
    (Default|SetThick _array_element_3 (/ (Variables|Components|GetTotalRadiusAngle) (Math|Conversions|ToFloat(Integer) (Variables|Components|GetTotalPieceNum))))))

(fn CheckPlayerinTunnel
  (params (RelativeAngle :type Float%20%28single-precision%29))
  (bind _startangle (Variables|Components|GetStartAngle))
  (bind _totalradiusangle (Variables|Components|GetTotalRadiusAngle))
  (bind _returnvalue (+ _startangle _totalradiusangle))
  (return (or (and (>= RelativeAngle _startangle) (<= RelativeAngle _returnvalue)) (<= RelativeAngle (- _returnvalue 3.6e+02)))))

(fn PlayerRespawn
  (bind _returnvalue (Game|GetPlayerCharacter 0))
  (Transformation|SetActorRelativeLocation _returnvalue (Transformation|GetWorldLocation (Variables|/Script/Engine.Actor|GetRootComponent (Variables|Components|GetPlayerRespawnActor))))
  (Variables|/Script/Engine.MovementComponent|SetVelocity (Pawn|GetMovementComponent _returnvalue) "0, 0, 0")
  (Variables|Components|SetSelfRotateOffsetAngleBase -1.8e+02)
  (Variables|Components|SetSelfRotateOffsetAngle -1.8e+02)
  (CallFunction|UpdateView))