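; Room 12 puzzle controller that builds a centered row of typed buttons on a screen and lets two be paired.
; TryToSelect ignores type 0, connected, blocked or disabled cases; a second pick connects if types differ, or match when ConnectType is set.
; A connection recolors both buttons, spawns a line, fires OnConnect and blocks further pairs unless AllowMultiConnect.
; Reset clears selections, connections and lines, then fires OnReset, unless Disabled.
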(event Custom|OnReset_Event)

(event Custom|OnConnect_Event
  (params (Smaller :type Integer) (Larger :type Integer)))

(event EventBeginPlay
  (Utilities|FlowControl|Sequence
    (:then_0
      ;[1 1 1] Construction
      (Actor|SetOwner (Variables|/Script/Engine.ChildActorComponent|GetChildActor (Variables|Default|GetResetButton)) self)
      (for (_array_element _array_index) (Variables|Components|GetButtonTypes)
        (bind _returnvalue (Game|SpawnActorfromClass "/Game/BP/BP_Room12_ControllerButton.BP_Room12_ControllerButton_C" (Math|Transform|MakeTransform "0, 0, 0") "Undefined" 0 0))
        (Variables|/Game/BP/BP_Room12_ControllerButton.BP_Room12_ControllerButton_C|SetButtonType _returnvalue _array_element)
        (Transformation|AttachComponentToComponent _returnvalue (Variables|Default|GetScreenScene) "None" "KeepRelative" "KeepRelative" "KeepRelative" true)
        (Transformation|SetActorRelativeLocation _returnvalue (Math|Vector|MakeVector 0.0 (Utilities|GetButtonOffsetfromIndex (Math|Conversions|ToFloat(Integer) _array_index)) 0.0))
        (Actor|SetOwner _returnvalue self)
        (Utilities|Array|Add (Variables|Components|GetButtons) _returnvalue)))
    (:then_1
      (EventDispatchers|BindEventtoOnReset (delegate Custom|OnReset_Event)))
    (:then_2
      (EventDispatchers|BindEventtoOnConnect (delegate Custom|OnConnect_Event)))
    (:then_3
      (CallFunction|Reset))))

(fn ConstructionScript)

(fn TrytoSelect
  (params (Button :type BP%20Room%2012%20Controller%20Button%20Object%20Reference))
  (bind _buttons (Variables|Components|GetButtons))
  (bind _selectedindex (Variables|Components|GetSelectedIndex))
  (bind _selectedindex_2 (Variables|Components|GetSelectedIndex))
  (bind _returnvalue (Utilities|Array|FindItem _buttons Button))
  (bind _output (Utilities|Array|Get(acopy) _selectedindex_2))
  (bind _output_2 (Utilities|Array|Get(acopy) _selectedindex_2 1))
  (if (== _returnvalue -1)
    (Development|PrintString "Button NOT FOUND")
    (elif (not (Math|Boolean|ORBoolean (and (Variables|Components|GetBlocked) (not (Variables|Components|GetAllowMultiConnect))) (== (Utilities|Array|Get(acopy) (Variables|Components|GetButtonTypes) _returnvalue) 0) (Utilities|Array|ContainsItem (Variables|Components|GetConnectedIndex) _returnvalue) (Variables|Components|GetDisabled)))
      (LocalVariables|SetButtonIndex _returnvalue)
      (Rendering|Material|SetMaterial (Variables|/Game/BP/BP_Room12_ControllerButton.BP_Room12_ControllerButton_C|GetButton Button) 0 (Variables|Components|GetButtonSelectedMat))
      (Utilities|Array|AddUnique (Variables|Components|GetSelectedIndex) (LocalVariables|GetButtonIndex))
      (if (>= (Utilities|Array|Length _selectedindex) 2)
        (LocalVariables|SetSuccessFlag true)
        (LocalVariables|SetSuccessFlag (and (Class|KismetMathLibrary|XORBoolean (!= (Utilities|GetButtonTypefromIndex (Utilities|Array|Get(acopy) _selectedindex 1)) (Utilities|GetButtonTypefromIndex (Utilities|Array|Get(acopy) _selectedindex))) (Variables|Components|GetConnectType)) (LocalVariables|GetSuccessFlag)))
        (Utilities|FlowControl|Sequence
          (:then_0
            (if (LocalVariables|GetSuccessFlag)
              (for _array_element (Variables|Components|GetSelectedIndex)
                (Rendering|Material|SetMaterial (Variables|/Game/BP/BP_Room12_ControllerButton.BP_Room12_ControllerButton_C|GetButton (Utilities|Array|Get(acopy) (Variables|Components|GetButtons) _array_element)) 0 (Utilities|Array|Get(acopy) (Variables|Components|GetButtonConnectMat) (Utilities|GetButtonTypefromIndex _array_element))))
              (Variables|Components|SetBlocked true)
              (Utilities|Array|AppendArray (Variables|Components|GetConnectedIndex) (Variables|Components|GetSelectedIndex))
              (CallFunction|AddLine (Math|Conversions|ToFloat(Integer) _output) (Math|Conversions|ToFloat(Integer) _output_2))
              (Default|CallOnConnect (Math|Integer|Min(Integer) _output _output_2) (Math|Integer|Max(Integer) _output _output_2))
              (else
                (for _array_element_2 (Variables|Components|GetSelectedIndex)
                  (Rendering|Material|SetMaterial (Variables|/Game/BP/BP_Room12_ControllerButton.BP_Room12_ControllerButton_C|GetButton (Utilities|Array|Get(acopy) (Variables|Components|GetButtons) _array_element_2)) 0 (Utilities|Array|Get(acopy) (Variables|Components|GetButtonNormalMat) (Utilities|GetButtonTypefromIndex _array_element_2)))))))
          (:then_1
            (Utilities|Array|Clear (Variables|Components|GetSelectedIndex))))))))

(fn Reset
  (if (not (Variables|Components|GetDisabled))
    (for (_array_element _array_index) (Variables|Components|GetButtons)
      (Rendering|Material|SetMaterial (Variables|/Game/BP/BP_Room12_ControllerButton.BP_Room12_ControllerButton_C|GetButton _array_element) 0 (Utilities|Array|Get(acopy) (Variables|Components|GetButtonNormalMat) (Utilities|GetButtonTypefromIndex _array_index))))
    (Utilities|Array|Clear (Variables|Components|GetSelectedIndex))
    (Variables|Components|SetBlocked false)
    (Utilities|Array|Clear (Variables|Components|GetConnectedIndex))
    (for _array_element_2 (Variables|Components|GetLines)
      (Actor|DestroyActor _array_element_2))
    (Utilities|Array|Clear (Variables|Components|GetLines))
    (Default|CallOnReset)))

(fn AddLine
  (params (IndexA :type Float%20%28single-precision%29) (IndexB :type Float%20%28single-precision%29))
  (bind _returnvalue (Math|Float|Round IndexA))
  (bind _buttonconnectmat (Variables|Components|GetButtonConnectMat))
  (bind _button_type (Utilities|GetButtonTypefromIndex _returnvalue))
  (bind _returnvalue_2 (Game|SpawnActorfromClass "/Game/BP/BP_Room12_ControllerLine.BP_Room12_ControllerLine_C" (Math|Transform|MakeTransform "0, 0, 0") "Undefined" self 0))
  (Transformation|AttachComponentToComponent _returnvalue_2 (Variables|Default|GetScreenScene) "None" "KeepRelative" "KeepRelative" "KeepRelative" true)
  (Default|SetPos _returnvalue_2 (Utilities|GetButtonOffsetfromIndex IndexA) (Utilities|GetButtonOffsetfromIndex IndexB))
  (Default|SetMat _returnvalue_2 (select (== _button_type (Utilities|GetButtonTypefromIndex (Math|Float|Round IndexB))) (Utilities|Array|Get(acopy) _buttonconnectmat _button_type) (Utilities|Array|Get(acopy) _buttonconnectmat)))
  (Utilities|Array|Add (Variables|Components|GetLines) _returnvalue_2))