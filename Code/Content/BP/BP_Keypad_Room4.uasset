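; Keypad lock for Room 4 that spawns a row of button actors on BeginPlay, three starting as letters and five as digits.
; ChangeNumber cycles a button through A–H or 0–7 by character code while locked, or afterwards if ChangeAfterUnlock allows.
; Each change fires OnPasswordChange, whose handler prints the concatenated input.
; The password check, unlock and door-opening logic in ChangeNumber is disconnected and never runs.
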(event Custom|OnPasswordChange_Event
  (bind _password (CallFunction|GetInputPassword))
  (Development|PrintString _password))

(event EventBeginPlay
  (Utilities|FlowControl|Sequence
    (:then_0
      (CallFunction|AddButton 3 "A")
      (CallFunction|AddButton 5 "0"))
    (:then_1
      (EventDispatchers|BindEventtoOnPasswordChange (delegate Custom|OnPasswordChange_Event)))))

(fn ConstructionScript)

(fn ChangeNumber
  (params (Index :type Integer))
  (bind _buttons (Variables|Components|GetButtons))
  (bind _output (Utilities|Array|Get(acopy) _buttons Index))
  (bind _number (Variables|/Game/BP/BP_KeypadButton_Full.BP_KeypadButton_Full_C|GetNumber _output))
  (bind _returnvalue (Utilities|String|GetCharacterasNumber _number))
  (if (Variables|Components|GetisLocked)
    (Default|SetNumber _output (select (and (<= _returnvalue 57) (>= _returnvalue 48)) (Utilities|String|ToString(Integer) (Math|Integer|%(Integer) (+ (- _returnvalue 48) 1) 8)) (Utilities|Select :Index (- _returnvalue 65) :Option%200 "B" :Option%201 "C" :Option%202 "D" :Option%203 "E" :Option%204 "F" :Option%205 "G" :Option%206 "H" :Option%207 "A")) :!label _label)
    (Default|CallOnPasswordChange)
    (elif (Variables|组件|GetChangeAfterUnlock)
      (goto _label))))

(fn GetInputPassword
  (for _array_element (Variables|Components|GetButtons)
    (LocalVariables|SetRes (Utilities|String|Append (LocalVariables|GetRes) (Variables|/Game/BP/BP_KeypadButton_Full.BP_KeypadButton_Full_C|GetNumber _array_element))))
  (return (LocalVariables|GetRes)))

(fn AddButton
  (params (NumOfDigits :type Integer) (InitValue :type String))
  (bind _buttons (Variables|Components|GetButtons))
  ;[1 1 1] Construct Buttons
  (for _index (range 0 (- NumOfDigits 1))
    (bind _returnvalue (Game|SpawnActorfromClass "/Game/BP/BP_KeypadButton_Full.BP_KeypadButton_Full_C" (Math|Transform|MakeTransform "0, 0, 0") "Undefined" 0 0))
    (bind _returnvalue_2 (Utilities|Array|Add _buttons _returnvalue))
    (Variables|/Game/BP/BP_KeypadButton_Full.BP_KeypadButton_Full_C|SetIndexInParent (Utilities|Array|Get(acopy) _buttons _returnvalue_2) _returnvalue_2)
    (Variables|/Game/BP/BP_KeypadButton_Full.BP_KeypadButton_Full_C|SetParent (Utilities|Array|Get(acopy) _buttons _returnvalue_2) self)
    (Default|SetNumber (Utilities|Array|Get(acopy) _buttons _returnvalue_2) InitValue)
    (Default|SetCoord (Utilities|Array|Get(acopy) _buttons _returnvalue_2) (Math|Vector2D|MakeVector2D (+ (- (Math|Conversions|ToFloat(Integer) _returnvalue_2) (/ (Math|Conversions|ToFloat(Integer) (- (Variables|Components|GetTotalNum) 1)) 2.0)) (* (Math|Integer|%(Integer) _returnvalue_2 2) -0.085)) 0.0))))