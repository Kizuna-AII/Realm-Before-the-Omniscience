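; Player controller that lets the player reverse gravity with the G key.
; G toggles the reversed state, negates jump velocity, switches walkable floor angle, then triggers a jump.
; Every Tick adds a signed GravityScale vector plus a constant upward offset to the pawn's velocity, faking gravity manually.
; While reversed, polled W/S keys add forward/backward pushes along the camera's flattened forward direction, with debug prints.
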(event EventBeginPlay)

(event EventTick
  (params (DeltaSeconds :type Float%20%28single-precision%29))
  (bind _returnvalue (Game|Player|GetPlayerPawn 0))
  (bind _realgravity (CallFunction|GetRealGravity))
  (Variables|/Script/Engine.MovementComponent|SetVelocity (Pawn|GetMovementComponent _returnvalue) (+ _realgravity (Transformation|GetVelocity _returnvalue) "0,0,20.000000")))

(event Input|KeyboardEvents|G
  (params (Key :type Key%20Structure :default "None"))
  (bind _returnvalue (Game|GetPlayerCharacter 0))
  (:Pressed
    (CallFunction|Reverse)
    (Character|Jump _returnvalue)
    (Development|PrintString (Utilities|String|ToString(Float) (Variables|/Script/Engine.CharacterMovementComponent|GetJumpZVelocity (Variables|/Script/Engine.Character|GetCharacterMovement _returnvalue))))))

(fn ConstructionScript)

(fn Reverse
  (bind _returnvalue (Game|GetPlayerCharacter 0))
  (bind _charactermovement (Variables|/Script/Engine.Character|GetCharacterMovement _returnvalue))
  (bind _output_get (Variables|Default|SetisReverse (not (Variables|Default|GetisReverse))))
  (Variables|/Script/Engine.CharacterMovementComponent|SetJumpZVelocity _charactermovement (- 0.0 (Variables|/Script/Engine.CharacterMovementComponent|GetJumpZVelocity _charactermovement)))
  (if _output_get
    (Pawn|Components|CharacterMovement|SetWalkableFloorAngle _charactermovement 9e+01)
    (else
      (Pawn|Components|CharacterMovement|SetWalkableFloorAngle _charactermovement 45.0)))
  (Development|PrintString "Player Gravity Reversed!")
  (Variables|/Script/Engine.CharacterMovementComponent|SetbMaintainHorizontalGroundVelocity _charactermovement false))

(fn GetRealGravity
  (bind _returnvalue (Game|Player|IsInputKeyDown "W"))
  (bind _returnvalue_2 (Game|GetPlayerController 0))
  (bind _gravityscale (Variables|Default|GetGravityScale))
  (bind _playercameramanager (Variables|/Script/Engine.PlayerController|GetPlayerCameraManager _returnvalue_2))
  (bind _returnvalue_3 (Camera|GetCameraRotation _playercameramanager))
  (bind _returnvalue_4 (Math|Rotator|GetRotationXVector _returnvalue_3))
  (bind (_x _y) (Math|Vector|BreakVector _returnvalue_4))
  (bind _returnvalue_5 (Math|Vector2D|MakeVector2D _x _y))
  (bind _returnvalue_6 (Math|Vector2D|Vector2DLength _returnvalue_5))
  (bind _returnvalue_7 (/ _returnvalue_5 _returnvalue_6))
  (if (Variables|Default|GetisReverse)
    (LocalVariables|SetRes _gravityscale)
    (if _returnvalue
      (LocalVariables|SetRes (+ (LocalVariables|GetRes) (Math|Conversions|ToVector(Vector2D) (* _returnvalue_7 1e+01)))))
    (if (Game|Player|IsInputKeyDown "S")
      (LocalVariables|SetRes (+ (LocalVariables|GetRes) (Math|Conversions|ToVector(Vector2D) (* _returnvalue_7 -1e+01)))))
    (Development|PrintString (Utilities|String|ToString(Vector2d) _returnvalue_7) _returnvalue)
    (else
      (LocalVariables|SetRes (* _gravityscale -1.0))))
  (return (LocalVariables|GetRes)))